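; BP_CarAudioFromLocation is an actor that plays car audio from its placed location as an ambience sound.
; On BeginPlay it caches the first BP_AudioWizard in the level, then starts its Audio component after a short delay.
; Every tick it fades the component's volume linearly toward the wizard's master volume multiplied by its ambience volume, so it follows those settings.
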(event `self.ReceiveBeginPlay`
  (bind _outactors (`GameplayStatics.GetAllActorsOfClass` "/Game/Dev-Directory/Personal-Folders/Isaiah/Blueprints/BP_AudioWizard.BP_AudioWizard_C"))
  (set `self.AudioWizard` (`|GetArrayItem` _outactors))
  (`KismetSystemLibrary.Delay` 1.0)
  (`AudioComponent.Play` (`self.Audio`) 0.0))

(event `self.ReceiveTick`
  (params (DeltaSeconds :type "Float (single-precision)"))
  (bind _audiowizard (`self.AudioWizard`))
  (`AudioComponent.AdjustVolume` (`self.Audio`) 1.0 (* (`/Game/Dev-Directory/Personal-Folders/Isaiah/Blueprints/BP_AudioWizard.MasterVolume` _audiowizard) (`/Game/Dev-Directory/Personal-Folders/Isaiah/Blueprints/BP_AudioWizard.AmbienceVolume` _audiowizard)) "Linear"))

(fn `UserConstructionScript`)