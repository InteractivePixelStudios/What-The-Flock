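; Traffic light actor that cycles green, yellow and red and halts AI enemy cars while red.
; A self-recalling delayed event steps through the phases using per-color durations, with toggle functions setting light visibility.
; The toggles and phase changes also move the BoxRed trigger and switch its collision and activation.
; Cars overlapping BoxRed have their movement mode set to None, then Walking when the overlap ends.
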(event `self.ReceiveBeginPlay`
  (`self.SetTrafficLightColor` (`self.StartingColor`)))

(event `SetTrafficLightColor`
  (params (TrafficLightColor :type "/Game/Dev-Directory/Personal-Folders/Alex/AlexTestLevel/TrafficSystem/TrafficLight/E_TrafficLightColorEnum Enum" :default "NewEnumerator0"))
  (bind _output_get (set `self.trafficLightColors` TrafficLightColor))
  (switch `/Game/Dev-Directory/Personal-Folders/Alex/AlexTestLevel/TrafficSystem/TrafficLight/E_TrafficLightColorEnum` _output_get
    (:`NewEnumerator0`
      (`self.ToggleGreenLight` true)
      (`self.ToggleYellowLight` false)
      (`self.ToggleRedLight` false)
      (`KismetSystemLibrary.Delay` (`self.GreenLightDuration`))
      (`self.SetTrafficLightColor` "NewEnumerator1")
      (`PrimitiveComponent.SetCollisionEnabled` (`self.BoxRed`) "NoCollision"))
    (:`NewEnumerator1`
      (`self.ToggleGreenLight` false)
      (`self.ToggleYellowLight` true)
      (`self.ToggleRedLight` false)
      (`KismetSystemLibrary.Delay` 3.0)
      (`self.SetTrafficLightColor` "NewEnumerator2")
      (`PrimitiveComponent.SetCollisionEnabled` (`self.BoxRed`) "QueryAndPhysics"))
    (:`NewEnumerator2`
      (`self.ToggleGreenLight` false)
      (`self.ToggleYellowLight` false)
      (`self.ToggleRedLight` true)
      (`KismetSystemLibrary.Delay` (`self.RedLightDuration`))
      (`self.SetTrafficLightColor` "NewEnumerator0")
      (`PrimitiveComponent.SetCollisionEnabled` (`self.BoxRed`) "NoCollision"))))

(event `self.BoxRed.OnComponentBeginOverlap`
  (params (OverlappedComponent :type "PrimitiveComponent Object Reference") (OtherActor :type "Actor Object Reference") (OtherComp :type "PrimitiveComponent Object Reference") (OtherBodyIndex :type Integer) (bFromSweep :type Boolean) (SweepResult :type "HitResult Structure (by ref)"))
  (bind _asbp_aicar_enemy (cast `/Game/Dev-Directory/Personal-Folders/Alex/AlexTestLevel/TrafficSystem/BP_AICarEnemy` OtherActor))
  (`CharacterMovementComponent.SetMovementMode` (`Character.CharacterMovement` _asbp_aicar_enemy) "MOVE_None" 0))

(event `self.ReceiveTick`
  (params (DeltaSeconds :type "Float (single-precision)")))

(event `self.BoxRed.OnComponentEndOverlap`
  (params (OverlappedComponent :type "PrimitiveComponent Object Reference") (OtherActor :type "Actor Object Reference") (OtherComp :type "PrimitiveComponent Object Reference") (OtherBodyIndex :type Integer))
  (bind _asbp_aicar_enemy (cast `/Game/Dev-Directory/Personal-Folders/Alex/AlexTestLevel/TrafficSystem/BP_AICarEnemy` OtherActor))
  (`CharacterMovementComponent.SetMovementMode` (`Character.CharacterMovement` _asbp_aicar_enemy) "MOVE_Walking" 0))

(fn `EnableCollisions`
  (`/Engine/EditorBlueprintResources/StandardMacros.FlipFlop`
    (:`A`
      (`PrimitiveComponent.SetCollisionEnabled` (`self.BoxRed`) "QueryAndPhysics"))
    (:`B`
      (`PrimitiveComponent.SetCollisionEnabled` (`self.BoxRed`) "NoCollision"))))

(fn `ToggleGreenLight`
  (params (ToggleOn :type Boolean))
  (bind _boxred (`self.BoxRed`))
  (`SceneComponent.SetVisibility` (`self.green`) ToggleOn false)
  (`PrimitiveComponent.SetCollisionEnabled` _boxred "ProbeOnly")
  (`SceneComponent.SetVisibility` _boxred ToggleOn false)
  (`SceneComponent.K2_SetRelativeLocation` _boxred (-938.0 458.0 0.0) false false)
  (`ActorComponent.Deactivate` _boxred))

(fn `ToggleRedLight`
  (params (ToggleOn :type Boolean))
  (bind _boxred (`self.BoxRed`))
  (`SceneComponent.SetVisibility` (`self.red`) ToggleOn false)
  (`ActorComponent.SetActive` _boxred ToggleOn false)
  (`SceneComponent.SetVisibility` _boxred ToggleOn false)
  (set `self.IsRedLight` ToggleOn)
  (`SceneComponent.K2_SetRelativeLocation` _boxred (-938.0 458.0 -1317.0) false false)
  (`ActorComponent.Activate` _boxred false))

(fn `ToggleYellowLight`
  (params (ToggleOn :type Boolean))
  (`SceneComponent.SetVisibility` (`self.yellow`) ToggleOn false))

(fn `UserConstructionScript`)