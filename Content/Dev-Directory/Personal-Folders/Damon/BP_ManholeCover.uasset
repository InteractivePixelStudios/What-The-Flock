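; BP_ManholeCover is a boost actor that lifts the pigeon character upward when it overlaps the actor.
; The construction script sets the Box height from BoxExtent and offsets it so it rises from the root.
; On overlap, the Boost timeline lerps the pigeon's Z from its current location toward just above the box top, keeping X and Y, without sweeping for collision.
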(event `self.ReceiveActorBeginOverlap`
  (params (OtherActor :type "Actor Object Reference"))
  (bind (_returnvalue_x _returnvalue_y _returnvalue_z) (`KismetMathLibrary.BreakVector` (`BoxComponent.GetScaledBoxExtent` (`self.Box`))))
  (bind (_returnvalue_x_2 _returnvalue_y_2 _returnvalue_z_2) (`KismetMathLibrary.BreakVector` (`SceneComponent.K2_GetComponentLocation` (`self.DefaultSceneRoot`))))
  (bind _asbp_pigeon_character_ab (cast `/Game/Dev-Directory/Personal-Folders/Alex/AlexTestLevel/PlayerCharacter/BP_PigeonCharacter_AB` OtherActor))
  (bind (_direction _newtrack_0) (`Timeline|Boost` :!via `PlayFromStart`)
    (:`Update`
      (bind (_returnvalue_x_3 _returnvalue_y_3) (`KismetMathLibrary.BreakVector` (`self.K2_GetActorLocation` _asbp_pigeon_character_ab)))
      (`self.K2_SetActorLocation` _asbp_pigeon_character_ab (`KismetMathLibrary.VLerp` (`self.K2_GetActorLocation` _asbp_pigeon_character_ab) (`KismetMathLibrary.MakeVector` _returnvalue_x_3 _returnvalue_y_3 (+ _returnvalue_z_2 (* _returnvalue_z 2.0) 72.0)) _newtrack_0) false false))))

(fn `UserConstructionScript`
  (bind _box (`self.Box`))
  (bind _boxextent (`self.boxExtent`))
  (bind (_returnvalue_x _returnvalue_y) (`KismetMathLibrary.BreakVector` (`BoxComponent.GetScaledBoxExtent` _box)))
  (`BoxComponent.SetBoxExtent` _box (`KismetMathLibrary.MakeVector` _returnvalue_x _returnvalue_y _boxextent) true)
  (`SceneComponent.K2_SetRelativeLocation` _box (`KismetMathLibrary.MakeVector` 0.0 0.0 _boxextent) false false))