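; BP_AudioWizard is a level audio manager that plays world and weather ambience and gives AI enemy cars engine audio.
; On BeginPlay it assigns sounds from AudioLibrary to its audio components, then plays or stops ambience, wind, rain and thunder via boolean toggles.
; It spawns and attaches a BP_CarAudioFromLocation to each BP_AICarEnemy and sets its engine sound.
; Tick continually applies master and ambience volume, but only to Ambience1.
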(event `Ambience`
  ;[1 1 1] World Ambience
  (`self.SetAmbienceAudio`)
  (`self.Play Weather Ambience Audio`)
  (`self.PlayWorldAmbienceAudio`))

(event `self.ReceiveBeginPlay`
  ;[1 1 1] Begin Play
  (set `self.AudioLibrary` "/Game/Dev-Directory/Personal-Folders/Isaiah/Audio/1-AudioLibrary/AudioLibrary.AudioLibrary")
  (`self.Ambience`)
  (`self.GetAllCars`))

(event `GetAllCars`
  ;[1 1 1] Car Audio
  (bind _outactors (`GameplayStatics.GetAllActorsOfClass` "/Game/Dev-Directory/Personal-Folders/Alex/AlexTestLevel/TrafficSystem/BP_AICarEnemy.BP_AICarEnemy_C"))
  (for _array_element _outactors
    (bind _returnvalue (`|SpawnActorFromClass` "/Game/Dev-Directory/Personal-Folders/Isaiah/Audio/Cars/BP_CarAudioFromLocation.BP_CarAudioFromLocation_C" (`KismetMathLibrary.Conv_VectorToTransform` (`self.K2_GetActorLocation` _array_element)) "Undefined" "MultiplyWithRoot" _array_element null))
    (`self.K2_AttachToActor` _returnvalue _array_element "None" "SnapToTarget" "SnapToTarget" "KeepWorld" true)
    (`self.SetCarAudio`)))

(event `self.ReceiveTick`
  (params (DeltaSeconds :type "Float (single-precision)"))
  ;[1 1 1] Event Tick
  (`self.AdjustVolume`))

(event `SetCarAudio`
  ;[1 1 1] Car Audio
  (bind _outactors (`GameplayStatics.GetAllActorsOfClass` "/Game/Dev-Directory/Personal-Folders/Isaiah/Audio/Cars/BP_CarAudioFromLocation.BP_CarAudioFromLocation_C"))
  (for _array_element _outactors
    (`AudioComponent.SetSound` (`/Game/Dev-Directory/Personal-Folders/Isaiah/Audio/Cars/BP_CarAudioFromLocation.Audio` _array_element) (`/Game/Dev-Directory/Personal-Folders/Isaiah/Audio/1-AudioLibrary/BP_AL.CarEngineAudio` (`self.AudioLibrary`)))))

(event `AdjustVolume`
  ;[1 1 1] Volume
  (`AudioComponent.AdjustVolume` (`self.Ambience1`) 1.0 (* (`self.MasterVolume`) (`self.AmbienceVolume`)) "Linear"))

(fn `Play Weather Ambience Audio`
  (bind _wind (`self.Wind`))
  (bind _rain (`self.Rain`))
  (bind _thunder (`self.Thunder`))
  (`|ExecutionSequence`
    (:`then_0`
      (if (`self.Windy`)
        (`AudioComponent.Play` _wind 0.0)
        (else
          (`AudioComponent.Stop` _wind))))
    (:`then_1`
      (if (`self.Rainy`)
        (`AudioComponent.Play` _rain 0.0)
        (else
          (`AudioComponent.Stop` _rain))))
    (:`then_2`
      (if (`self.Thundery`)
        (`AudioComponent.Play` _thunder 0.0)
        (else
          (`AudioComponent.Stop` _thunder))))))

(fn `PlayWorldAmbienceAudio`
  (bind _ambience1 (`self.Ambience1`))
  (bind _ambience2 (`self.Ambience2`))
  (bind _ambience3 (`self.Ambience3`))
  (if (`self.PlayWorldAmbience`)
    (`|ExecutionSequence`
      (:`then_0`
        (`AudioComponent.Play` _ambience1 0.0))
      (:`then_1`
        (`AudioComponent.Play` _ambience2 0.0))
      (:`then_2`
        (`AudioComponent.Play` _ambience3 0.0)))
    (else
      (`|ExecutionSequence`
        (:`then_0`
          (`AudioComponent.Stop` _ambience1))
        (:`then_1`
          (`AudioComponent.Stop` _ambience2))
        (:`then_2`
          (`AudioComponent.Stop` _ambience3))))))

(fn `SetAmbienceAudio`
  (bind _audiolibrary (`self.AudioLibrary`))
  (`AudioComponent.SetSound` (`self.Ambience1`) (`/Game/Dev-Directory/Personal-Folders/Isaiah/Audio/1-AudioLibrary/BP_AL.Ambience1` _audiolibrary))
  (`AudioComponent.SetSound` (`self.Ambience2`) (`/Game/Dev-Directory/Personal-Folders/Isaiah/Audio/1-AudioLibrary/BP_AL.Ambience2` _audiolibrary))
  (`AudioComponent.SetSound` (`self.Ambience3`) (`/Game/Dev-Directory/Personal-Folders/Isaiah/Audio/1-AudioLibrary/BP_AL.Ambience3` _audiolibrary))
  (`AudioComponent.SetSound` (`self.Wind`) (`/Game/Dev-Directory/Personal-Folders/Isaiah/Audio/1-AudioLibrary/BP_AL.WindAmbience` _audiolibrary))
  (`AudioComponent.SetSound` (`self.Rain`) (`/Game/Dev-Directory/Personal-Folders/Isaiah/Audio/1-AudioLibrary/BP_AL.RainAmbience` _audiolibrary))
  (`AudioComponent.SetSound` (`self.Thunder`) (`/Game/Dev-Directory/Personal-Folders/Isaiah/Audio/1-AudioLibrary/BP_AL.ThunderAmbience` _audiolibrary)))

(fn `UserConstructionScript`)