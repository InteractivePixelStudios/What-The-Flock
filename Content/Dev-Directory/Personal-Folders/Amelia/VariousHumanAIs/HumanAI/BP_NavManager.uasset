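; BP_NavManager is a manager actor that hands out random navigation targets from the BP_NavNode actors in the level.
; Its construction script caches every BP_NavNode into NavNodeArray.
; GetRandomNavNode and GetRandomNavPOI return the transform of a random entry from the node and point-of-interest arrays.
; The logic that would fill NavPOIArray from PointOfInterest nodes is disconnected, and the event graph is empty.
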(fn `GetRandomNavNode`
  (returns (ReturnValue :type "Transform Structure (by ref)"))
  (bind _navnodearray (`self.NavNodeArray`))
  (return (`self.GetTransform` (`|GetArrayItem` _navnodearray (`KismetMathLibrary.RandomInteger` (`KismetArrayLibrary.Array_Length` _navnodearray))))))

(fn `GetRandomNavPOI`
  (returns (ReturnValue :type "Transform Structure (by ref)"))
  (bind _navpoiarray (`self.NavPOIArray`))
  (return (`self.GetTransform` (`|GetArrayItem` _navpoiarray (`KismetMathLibrary.RandomInteger` (`KismetArrayLibrary.Array_Length` _navpoiarray))))))

(fn `UserConstructionScript`
  (bind _outactors (`GameplayStatics.GetAllActorsOfClass` "/Game/Dev-Directory/Personal-Folders/Amelia/VariousHumanAIs/HumanAI/NavNodes/BP_NavNode.BP_NavNode_C"))
  (set `self.NavNodeArray` _outactors))