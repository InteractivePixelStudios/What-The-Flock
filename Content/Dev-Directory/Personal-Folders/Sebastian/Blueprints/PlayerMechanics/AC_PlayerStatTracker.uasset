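; Player component that tracks gameplay stats such as collectibles, consumables eaten, poops, enemies pooped on or evaded, completed missions and race times.
; Small setter, increment and add functions update each stat, with race times stored by race name.
; SetLoadedStats restores all stats at once and GetAllStats returns them together.
; GetPlayerAccuracy derives a rounded percentage from enemies pooped on over times pooped, without a zero check.
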(fn `AddCompletedMission`
  (params (MissionName :type String))
  (`KismetArrayLibrary.Array_Add` (`self.MissionsCompleted`) MissionName))

(fn `AddRaceTime`
  (params (RaceName :type String) (RaceTime :type "Float (double-precision)"))
  (`BlueprintMapLibrary.Map_Add` (`self.RaceTimes`) RaceName RaceTime))

(fn `GetAllStats`
  (returns (SeedsCollected :type Integer) (TrinketsCollected :type Integer) (ItemsCollected :type Integer) (ConsumablesEaten :type Integer) (TimesPooped :type Integer) (EnemiesPoopedOn :type Integer) (EnemiesEvaded :type Integer) (MissionsCompleted :type "Array of String") (RaceTimes :type "Map of String to Float (double-precision)"))
  (return (`self.SeedsCollected`) (`self.TrinketsCollected`) (`self.ItemsCollected`) (`self.ConsumablesEaten`) (`self.TimesPooped`) (`self.EnemiesPoopedOn`) (`self.EnemiesEvaded`) (`self.MissionsCompleted`) (`self.RaceTimes`)))

(fn `GetPlayerAccuracy`
  (returns (AccuracyPercentage :type Integer))
  (return (`KismetMathLibrary.Round` (* (/ (`KismetMathLibrary.Conv_IntToDouble` (`self.EnemiesPoopedOn`)) (`KismetMathLibrary.Conv_IntToDouble` (`self.TimesPooped`))) 100.0))))

(fn `IncrementConsumablesEaten`
  (`/Engine/EditorBlueprintResources/StandardMacros.IncrementInt` (`self.ConsumablesEaten`)))

(fn `IncrementEnemiesEvaded`
  (`/Engine/EditorBlueprintResources/StandardMacros.IncrementInt` (`self.EnemiesEvaded`)))

(fn `IncrementEnemiesPoopedOn`
  (`/Engine/EditorBlueprintResources/StandardMacros.IncrementInt` (`self.EnemiesPoopedOn`)))

(fn `IncrementItemsCollected`
  (`/Engine/EditorBlueprintResources/StandardMacros.IncrementInt` (`self.ItemsCollected`)))

(fn `IncrementTimesPooped`
  (`/Engine/EditorBlueprintResources/StandardMacros.IncrementInt` (`self.TimesPooped`)))

(fn `IncrementTrinketsCollected`
  (params (TrinketsGained :type Integer))
  (set `self.TrinketsCollected` (+ TrinketsGained (`self.TrinketsCollected`))))

(fn `SetLoadedStats`
  (params (Seeds :type Integer) (Trinkets :type Integer) (Items :type Integer) (Consumables :type Integer) (TimesPooped :type Integer) (EnemiesPooped :type Integer) (EnemiesEvaded :type Integer) (Missions :type "Array of String") (Races :type "Map of String to Float (double-precision)"))
  (set `self.SeedsCollected` Seeds)
  (set `self.TrinketsCollected` Trinkets)
  (set `self.ItemsCollected` Items)
  (set `self.ConsumablesEaten` Consumables)
  (set `self.TimesPooped` TimesPooped)
  (set `self.EnemiesPoopedOn` EnemiesPooped)
  (set `self.EnemiesEvaded` EnemiesEvaded)
  (set `self.MissionsCompleted` Missions)
  (set `self.RaceTimes` Races))

(fn `SetSeedsCollected`
  (params (Seeds :type Integer))
  (set `self.SeedsCollected` Seeds))