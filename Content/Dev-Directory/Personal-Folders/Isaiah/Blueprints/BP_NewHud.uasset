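; BP_NewHud creates and manages the player HUD and world map widgets for the pigeon character game.
; The M key swaps between HUD and map, also showing or hiding the WorldMapArrow.
; Each Tick drives the compass image's dynamic material rotation from the pigeon fly camera's yaw.
; UpdateHUD copies health, stamina, dooky and EXP from player stats into listener variables, relying on manual calls after stat changes.
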(event `self.ReceiveTick`
  (params (DeltaSeconds :type "Float (single-precision)"))
  (`self.SetCompass`))

(event `self.ReceiveBeginPlay`
  ;[1 1 1] On Begin - Create HUD and World Map Widgets.
  (`self.CreateHUD`)
  (`self.UpdateHUD`)
  (`SceneComponent.SetHiddenInGame` (`self.WorldMap_Arrow`) true false))

(event `Key|M`
  (params (Key :type "Key Structure"))
  ;[1 1 1] Button Listeners
  ;;[1 0.7618 0] World Map Toggle
  (:`Pressed`
    (if (`self.Is Map Open`)
      (`KismetSystemLibrary.PrintString` "M was presse")
      (`self.Toggle World Map OFF`)
      (else
        (`self.Toggle World Map ON`)))))

(event `Toggle World Map ON`
  ;[1 1 1] Toggle World Map
  (set `self.Is Map Open` true)
  (`Widget.SetVisibility` (`self.Player HUD`) "Hidden")
  (`SceneComponent.SetHiddenInGame` (`self.WorldMap_Arrow`) false false)
  (`Widget.SetVisibility` (`self.WorldMap`) "Visible")
  (`KismetSystemLibrary.PrintText` "Toggled Map On"))

(event `Toggle World Map OFF`
  ;[1 1 1] Toggle World Map
  (set `self.Is Map Open` false)
  (`Widget.SetVisibility` (`self.WorldMap`) "Hidden")
  (`SceneComponent.SetHiddenInGame` (`self.WorldMap_Arrow`) true false)
  (`Widget.SetVisibility` (`self.Player HUD`) "Visible")
  (`KismetSystemLibrary.PrintText` "Toggle Map Off"))

(event `UpdateHUD`
  ;[1 1 1] System that listens to the game stats and adjusts the Sliders as needed - UpdateHUD MUST be called when a stat changes.
  (set `self.HealthListener` (`/Game/Dev-Directory/Personal-Folders/Isaiah/Blueprints/BP_PlayerStats.Health` (`self.BP_PlayerStats`)))
  (set `self.StaminaListener` (`/Game/Dev-Directory/Personal-Folders/Isaiah/Blueprints/BP_PlayerStats.Stamina` (`self.BP_PlayerStats`)))
  (set `self.DookyListener` (`/Game/Dev-Directory/Personal-Folders/Isaiah/Blueprints/BP_PlayerStats.Dooky` (`self.BP_PlayerStats`)))
  (set `self.EXPListener` (`/Game/Dev-Directory/Personal-Folders/Isaiah/Blueprints/BP_PlayerStats.EXP` (`self.BP_PlayerStats`))))

(event `CreateHUD`
  ;[1 1 1] HUD & World Map Widget Creation
  (bind _returnvalue (`|CreateWidget` "/Game/Dev-Directory/Personal-Folders/Isaiah/PlayerHUD_Widget.PlayerHUD_Widget_C" (`GameplayStatics.GetPlayerController` 0)))
  (bind _output_get (set `self.Player HUD` _returnvalue))
  (bind _output_get_2 (set `self.Compass` _output_get))
  (`UserWidget.AddToViewport` _output_get_2 0)
  (bind _returnvalue_2 (`|CreateWidget` "/Game/Dev-Directory/Personal-Folders/Isaiah/WorldMap_Widget.WorldMap_Widget_C" (`GameplayStatics.GetPlayerController` 0)))
  (bind _output_get_3 (set `self.WorldMap` _returnvalue_2))
  (`UserWidget.AddToViewport` _output_get_3 0)
  (`Widget.SetVisibility` (`self.WorldMap`) "Hidden")
  (set `self.Is Map Open` false)
  (`KismetSystemLibrary.PrintText` "HUD and World Map have been created."))

(event `SetCompass`
  ;[1 1 1] Compass Logic
  (bind _asbp_pigeon_character_ab (cast `/Game/Dev-Directory/Personal-Folders/Alex/AlexTestLevel/PlayerCharacter/BP_PigeonCharacter_AB` (`GameplayStatics.GetPlayerCharacter` 0)))
  (bind _returnvalue (`Image.GetDynamicMaterial` (`/Game/Dev-Directory/Personal-Folders/Isaiah/PlayerHUD_Widget.CompassImage` (`self.Compass`))))
  (bind (_returnvalue_roll _returnvalue_pitch _returnvalue_yaw) (`KismetMathLibrary.BreakRotator` (`SceneComponent.K2_GetComponentRotation` (`/Game/Dev-Directory/Personal-Folders/Alex/AlexTestLevel/PlayerCharacter/BP_PigeonCharacter_AB.FlyCameraRef` _asbp_pigeon_character_ab))))
  (`MaterialInstanceDynamic.SetScalarParameterValue` _returnvalue "Compass Rotation" (/ _returnvalue_yaw 360.0)))

(fn `UserConstructionScript`)