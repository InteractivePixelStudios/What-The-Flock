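; Health pick-up actor that either restores or removes the pigeon character's health, depending on its RestoresHealth flag.
; Overlap caches the BP_PigeonCharacter_AB and prints a prompt to press E.
; The Pickup event calls DestroyActor, then passes HealthEffectValue to RestoreHealth or LoseHealth on that character's BPHealthSystemWK, with debug prints.
; The file contains no caller for Pickup, and a GetPlayerPawn cast path is left unconnected.
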(event `self.Pickup`
  (bind _healtheffectvalue (`self.HealthEffectValue`))
  ;[1 1 1] Checks to see if the player picked up the object and deletes it
  (`self.K2_DestroyActor`)
  ;;[1 1 1] debug message
  (`KismetSystemLibrary.PrintString` "item picked")
  ;[1 1 1] Sets the players speed/ this is where you impliment code for other effects.
  (if (`self.RestoresHealth`)
    (bind _bp_healthsystem_wk (`/Game/Dev-Directory/Personal-Folders/Alex/AlexTestLevel/PlayerCharacter/BP_PigeonCharacter_AB.BP_HealthSystem_WK` (stale `self.ReceiveActorBeginOverlap` _asbp_pigeon_character_ab)))
    (`/Game/Dev-Directory/Personal-Folders/Wesley/BluePrints_WK/BP_HealthSystem_WK.RestoreHealth` _bp_healthsystem_wk _healtheffectvalue)
    (`KismetSystemLibrary.PrintText` "health restored")
    (else
      (`/Game/Dev-Directory/Personal-Folders/Wesley/BluePrints_WK/BP_HealthSystem_WK.LoseHealth` _bp_healthsystem_wk _healtheffectvalue)
      (`KismetSystemLibrary.PrintText` "health lost"))))

(event `self.ReceiveActorBeginOverlap`
  (params (OtherActor :type "Actor Object Reference"))
  ;[1 1 1] Checks to see if the player is overlapping for input message
  (bind _asbp_pigeon_character_ab (cast `/Game/Dev-Directory/Personal-Folders/Alex/AlexTestLevel/PlayerCharacter/BP_PigeonCharacter_AB` OtherActor))
  (`KismetSystemLibrary.PrintText` "Press \"E\" to pickup"))

(fn `UserConstructionScript`)