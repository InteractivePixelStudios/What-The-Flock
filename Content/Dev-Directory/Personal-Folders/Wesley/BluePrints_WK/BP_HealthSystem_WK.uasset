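; Health component for the pigeon character, tracking current and max health as integers and handling death.
; Current health starts at max, and healing or damage is clamped between zero and max.
; Reaching zero fires OnBirbDeath, which casts the owner to BP_PigeonCharacter_AB, turns off its UI and starts its respawn system.
; Leveling up raises both max and current health by a fixed amount.
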(event `self.ReceiveBeginPlay`
  ;[1 1 1] At start, set Current Health to Max Health
  (set `self.HealthCurrent` (`self.HealthMax`)))

(event `self.ReceiveTick`
  (params (DeltaSeconds :type "Float (single-precision)")))

(event `/Game/Dev-Directory/Personal-Folders/Jacob-EXP/XP-Content/BPI_XPInterface_JS.OnLevelUp`
  ;[1 1 1] On Level Up
  (`self.IncreaseMaxHealth` 2))

(event `On Birb Death`
  ;[1 1 1] On Birb Death
  (bind _asbp_pigeon_character_ab (cast `/Game/Dev-Directory/Personal-Folders/Alex/AlexTestLevel/PlayerCharacter/BP_PigeonCharacter_AB` (`self.GetOwner`)))
  (`/Game/Dev-Directory/Personal-Folders/Alex/AlexTestLevel/PlayerCharacter/BP_PigeonCharacter_AB.TurnUIOnOff` _asbp_pigeon_character_ab false)
  (`/Game/Dev-Directory/Personal-Folders/Wesley/BluePrints_WK/BP_RespawnSystem_WK.Start Respawn` (`/Game/Dev-Directory/Personal-Folders/Alex/AlexTestLevel/PlayerCharacter/BP_PigeonCharacter_AB.BP_RespawnSystem_WK` _asbp_pigeon_character_ab)))

(fn `IncreaseMaxHealth`
  (params (MaxHealthIncrease :type Integer :default 2))
  ;[1 1 1] When called, increases max health by the input value and restores that same value to current health
  (bind _output_get (set `self.HealthMax` (+ (`self.HealthMax`) MaxHealthIncrease))) ; Set Max Health to new value
  (set `self.HealthCurrent` (+ (`self.HealthCurrent`) (`local.MaxHealthIncrease`))) ; set new value to Current Health
  ;[1 0.7157 0.04971] Debug
  (`KismetSystemLibrary.PrintText` "Max Health increased to ")
  (`KismetSystemLibrary.PrintText` (`KismetTextLibrary.Conv_IntToText` _output_get)))

(fn `LoseHealth`
  (params (DamageTaken :type Integer))
  ;[1 1 1] Get Damage Taken and subtract it from current health, making sure it doesnt go below 0, and set the value to Current Health
  (bind _output_get (set `self.HealthCurrent` (`KismetMathLibrary.Clamp` (- (`self.HealthCurrent`) DamageTaken) 0 (`self.HealthMax`)))) ; Set new Current Health
  (if (not (> _output_get 0))
    (`self.On Birb Death`)))

(fn `RestoreHealth`
  (params (HealthRestored :type Integer))
  (bind _returnvalue (`KismetMathLibrary.Clamp` (+ HealthRestored (`self.HealthCurrent`)) 0 (`self.HealthMax`)))
  ;[1 1 1] Get Health restored and add it to current health, making sure it doesnt go above Max Health, and set the value to Current Health
  (set `self.HealthCurrent` _returnvalue) ; Set new Current Health
  ;[1 0.7157 0.04971] Debug
  (`KismetSystemLibrary.PrintText` "health restored by ")
  (`KismetSystemLibrary.PrintText` (`KismetTextLibrary.Conv_IntToText` _returnvalue)))