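; Respawn component for the pigeon player character that lets the player respawn at a selected respawn point.
; StartRespawn shows lazily created map and pick-respawn widgets, switches input to UI-only and points the camera at the level's BP_RespawnManager.
; RespawnPlayer moves the pawn just above the manager's current point, removes the widgets, returns camera, input and HUD to the player, and restores full health.
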(event `self.ReceiveBeginPlay`
  (bind _returnvalue (`GameplayStatics.GetActorOfClass` "/Game/Dev-Directory/Personal-Folders/Amelia/RespawnSystem/BP_RespawnManager.BP_RespawnManager_C"))
  (set `self.RespawnManager` _returnvalue)
  (bind _asbp_pigeon_character_ab (cast `/Game/Dev-Directory/Personal-Folders/Alex/AlexTestLevel/PlayerCharacter/BP_PigeonCharacter_AB` (`self.GetOwner`)))
  (set `self.Player Ref` _asbp_pigeon_character_ab))

(event `Respawn Player`
  (bind _returnvalue (`GameplayStatics.GetPlayerController` 0))
  (bind _player_ref (`self.Player Ref`))
  (bind _bp_healthsystem_wk (`/Game/Dev-Directory/Personal-Folders/Alex/AlexTestLevel/PlayerCharacter/BP_PigeonCharacter_AB.BP_HealthSystem_WK` _player_ref))
  ;[0.231 0.1121 0.5521] Teleports player to selected respawn point
  (bind _newparam (`/Game/Dev-Directory/Personal-Folders/Amelia/RespawnSystem/BP_RespawnManager.GetCurrentRespawnPoint` (`self.RespawnManager`)))
  (`Actor.K2_SetActorLocation` (`GameplayStatics.GetPlayerPawn` 0) (`KismetMathLibrary.MakeVector` (.x (`Actor.K2_GetActorLocation` _newparam)) (.y (`Actor.K2_GetActorLocation` _newparam)) (+ (.z (`Actor.K2_GetActorLocation` _newparam)) 50.0)) false false)
  (`Widget.RemoveFromParent` (`self.Debug Reference`))
  (`Widget.RemoveFromParent` (`self.Pause Reference`))
  ;[1 1 1] Returns camera and control to the player
  (set `self.IsRespawning` false)
  (set `PlayerController.bShowMouseCursor` false _returnvalue)
  (`WidgetBlueprintLibrary.SetInputMode_GameOnly` _returnvalue)
  (`Actor.EnableInput` _player_ref _returnvalue)
  (`PlayerController.SetViewTargetWithBlend` _returnvalue _player_ref 0.0 "VTBlend_Linear" 0.0 false)
  (`/Game/Dev-Directory/Personal-Folders/Alex/AlexTestLevel/PlayerCharacter/BP_PigeonCharacter_AB.TurnUIOnOff` _player_ref true)
  (`/Game/Dev-Directory/Personal-Folders/Wesley/BluePrints_WK/BP_HealthSystem_WK.RestoreHealth` _bp_healthsystem_wk (`/Game/Dev-Directory/Personal-Folders/Wesley/BluePrints_WK/BP_HealthSystem_WK.HealthMax` _bp_healthsystem_wk)))

(event `Start Respawn`
  (bind _returnvalue (`GameplayStatics.GetPlayerController` 0))
  (bind _debug_reference (`self.Debug Reference`))
  (bind _pause_reference (`self.Pause Reference`))
  (`/Engine/EditorBlueprintResources/StandardMacros.IsValid` (`self.Pause Reference`)
    (:`Is Valid`
      _)
    (:`Is Not Valid`
      ;[1 1 1] If widget doesn't exist, make one
      (bind _returnvalue_2 (`|CreateWidget` "/Game/Dev-Directory/Personal-Folders/Amelia/RespawnSystem/UW_RespawnMap.UW_RespawnMap_C"))
      (set `self.Pause Reference` _returnvalue_2)
      (bind _returnvalue_3 (`|CreateWidget` "/Game/Dev-Directory/Personal-Folders/Amelia/RespawnSystem/UW_PickRespawn.UW_PickRespawn_C"))
      (set `self.Debug Reference` _returnvalue_3)))
  (if (not (`self.IsRespawning`))
    (`/Game/Dev-Directory/Personal-Folders/Amelia/RespawnSystem/UW_RespawnMap.Refresh List` _pause_reference)
    (`UserWidget.AddToViewport` _pause_reference 0)
    (`UserWidget.AddToViewport` _debug_reference 0)
    ;[1 1 1] Takes away player control and enters respawn UI
    (set `self.IsRespawning` true)
    (set `PlayerController.bShowMouseCursor` true _returnvalue)
    (`WidgetBlueprintLibrary.SetInputMode_UIOnlyEx` _returnvalue _debug_reference)
    (`Actor.EnableInput` _returnvalue null)
    (`PlayerController.SetViewTargetWithBlend` _returnvalue (`self.RespawnManager`) 0.0 "VTBlend_Linear" 0.0 false)))