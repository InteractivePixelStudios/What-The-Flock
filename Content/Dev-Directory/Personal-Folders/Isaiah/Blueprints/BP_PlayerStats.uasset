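; BP_PlayerStats holds the player's Health, Stamina, Dooky and EXP values, with a debug key to randomize them.
; BeginPlay sets starting values on a 0–100 scale.
; Pressing R overrides all four with random fractions up to 1.0, a different scale from the defaults.
; Releasing R prints an override warning and calls UpdateHUD on all BP_CustomPawn actors.
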(event `self.ReceiveBeginPlay`
  (set `self.Health` 100.0)
  (set `self.Stamina` 100.0)
  (set `self.Dooky` 50.0)
  (set `self.EXP` 0.0))

(event `Key|R`
  (params (Key :type "Key Structure"))
  (bind _returnvalue (`KismetMathLibrary.RandomFloatInRange` 0.05 1.0))
  (:`Pressed`
    (set `self.Health` _returnvalue)
    (set `self.Stamina` _returnvalue)
    (set `self.Dooky` _returnvalue)
    (set `self.EXP` _returnvalue))
  (:`Released`
    (`KismetSystemLibrary.PrintString` "WARNING: Stat Overide Command Has Been Run." true true (struct :`G` 0.66 :`B` 1.0 :`A` 1.0) 3.0)
    (bind _outactors (`GameplayStatics.GetAllActorsOfClass` "/Game/Dev-Directory/Personal-Folders/Isaiah/Blueprints/BP_CustomPawn.BP_CustomPawn_C"))
    (`/Game/Dev-Directory/Personal-Folders/Isaiah/Blueprints/BP_CustomPawn.UpdateHUD` _outactors)))