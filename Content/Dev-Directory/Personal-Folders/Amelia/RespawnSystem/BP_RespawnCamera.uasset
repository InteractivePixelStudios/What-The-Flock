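; BP_RespawnCamera is a camera actor for the respawn system that moves horizontally to a requested location.
; MoveCameraLerp glides there over a one-second timeline, interpolating from the current position on each update, while MoveCamera teleports instantly.
; Both events change only X and Y, keeping the actor's height, and move without sweeping.
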(event `MoveCameraLerp`
  (params (NewLocation :type "Vector Structure"))
  (bind _returnvalue (`self.K2_GetActorLocation`))
  ;[1 1 1] 0-1 in 1 Second
  (bind (_direction _transition) (`Timeline|Timeline` :!via `PlayFromStart`)
    (:`Update`
      (`self.K2_SetActorLocation` (`KismetMathLibrary.MakeVector` (.x (`KismetMathLibrary.VLerp` _returnvalue NewLocation _transition)) (.y (`KismetMathLibrary.VLerp` _returnvalue NewLocation _transition)) (.z _returnvalue)) false true))))

(event `MoveCamera`
  (params (`New Location` :type "Vector Structure"))
  (`self.K2_SetActorLocation` (`KismetMathLibrary.MakeVector` (.x `New Location`) (.y `New Location`) (.z (`self.K2_GetActorLocation`))) false true))

(fn `UserConstructionScript`)