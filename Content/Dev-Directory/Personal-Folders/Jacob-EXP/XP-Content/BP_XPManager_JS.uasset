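; Experimental XP manager Blueprint that tracks the player's XP and level, with debug prints throughout.
; IncreaseXP feeds CollectXP, which adds XP until max level and calls LevelUp once when the threshold is reached.
; LevelUp carries over surplus XP, increments the level and calls OnLevelUp on each registered listener.
; The threshold increase currently adds zero, and XP gained at max level is discarded.
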(event `/Game/Dev-Directory/Personal-Folders/Jacob-EXP/XP-Content/BPI_XPInterface_JS.IncreaseXP`
  (params (`XP amount` :type Integer))
  (`self.CollectXP` `XP amount`))

(event `/Game/Dev-Directory/Personal-Folders/Jacob-EXP/XP-Content/BPI_XPInterface_JS.OnLevelUp`
  (`KismetSystemLibrary.PrintString` "Successfully triggered On Level Up Interface to XP Manager"))

(fn `CollectXP`
  (params (XPAmount :type Integer))
  ;[1 1 1] XP Increase Debug
  (`KismetSystemLibrary.PrintString` "XP Added!" true true (struct :`G` 1.0 :`B` 0.004862 :`A` 1.0) 10.0)
  (`KismetSystemLibrary.PrintString` (`KismetStringLibrary.Conv_IntToString` XPAmount) true true (struct :`G` 1.0 :`B` 0.223108 :`A` 1.0) 10.0)
  ;[1 1 1] XP Increase Override if max level is reached
  (if (== (`self.PlayerLevel`) (`self.MaxLevel`))
    (`KismetSystemLibrary.PrintString` "Max Level Reached. What do with extra xp?")
    (else
      ;[1 1 1] Increase Current XP
      (bind _output_get (set `self.CurrentXP` (+ XPAmount (`self.CurrentXP`))))
      ;[1 1 1] Check if XP Threshold reached
      (if (>= _output_get (`self.XPThreshold`))
        (`self.LevelUp`)))))

(fn `LevelUp`
  (set `self.CurrentXP` (- (`self.CurrentXP`) (`self.XPThreshold`))) ; Suibtracts the XP threshold from current xp. (e.g if you have 5 xp and need 4 to level up, you will have 1 carry over.)
  (bind _output_get (set `self.PlayerLevel` (+ (`self.PlayerLevel`) 1))) ; increment player lvl
  (`KismetSystemLibrary.PrintString` "Level Incremented to:")
  (`KismetSystemLibrary.PrintString` (`KismetStringLibrary.Conv_IntToString` _output_get))
  (bind _output_get_2 (set `self.XPThreshold` (+ (`self.XPThreshold`) 0.0))) ; Increases the XP Threshold required for the next level
  (`KismetSystemLibrary.PrintString` "XP Threshold is now:")
  (`KismetSystemLibrary.PrintString` (`KismetStringLibrary.Conv_DoubleToString` _output_get_2))
  ;[1 1 1] Calling each Component on pigeon that has XP Interface
  (for _array_element (`self.RegisteredListeners`)
    (`/Game/Dev-Directory/Personal-Folders/Jacob-EXP/XP-Content/BPI_XPInterface_JS.OnLevelUp` _array_element)))