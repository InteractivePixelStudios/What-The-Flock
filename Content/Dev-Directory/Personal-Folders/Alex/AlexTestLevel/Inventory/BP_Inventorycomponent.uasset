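; BP_Inventorycomponent is an inventory component that holds items and drives the player inventory widget.
; On BeginPlay it creates WB_PlayerInventory, sizes the Items array to four slots and passes itself to the widget to load.
; The open-inventory input toggles the widget on and off the viewport.
; Pressing E runs a debug-drawn sphere trace near the player's feet, but the result is not used yet.
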(event `self.ReceiveBeginPlay`
  (bind _returnvalue (`|CreateWidget` "/Game/Dev-Directory/Personal-Folders/Alex/AlexTestLevel/Inventory/WB_PlayerInventory.WB_PlayerInventory_C"))
  (set `self.InventoryWidget` _returnvalue)
  (`KismetArrayLibrary.Array_Resize` (`self.Items`) 4)
  (`/Game/Dev-Directory/Personal-Folders/Alex/AlexTestLevel/Inventory/WB_PlayerInventory.LoadInventory` (`self.InventoryWidget`) self))

(event `EnhancedInput|/Game/Dev-Directory/Personal-Folders/Alex/AlexTestLevel/EnhancedInput/IA_OpenInventory`
  (params (ActionValue :type Boolean) (ElapsedSeconds :type "Float (double-precision)") (TriggeredSeconds :type "Float (double-precision)") (InputAction :type "InputAction Object Reference" :default "/Game/Dev-Directory/Personal-Folders/Alex/AlexTestLevel/EnhancedInput/IA_OpenInventory.IA_OpenInventory"))
  (bind _inventorywidget (`self.InventoryWidget`))
  (:`Completed`
    (if (`Widget.IsVisible` (`self.InventoryWidget`))
      (`Widget.RemoveFromParent` _inventorywidget)
      (else
        (`UserWidget.AddToViewport` _inventorywidget 0)))))

(event `Key|E`
  (params (Key :type "Key Structure"))
  (bind _returnvalue (- (`Actor.K2_GetActorLocation` (`GameplayStatics.GetPlayerCharacter` 0)) (0.0 0.0 65.0)))
  (:`Pressed`
    (`KismetSystemLibrary.SphereTraceSingle` :`Start` _returnvalue :`End` _returnvalue :`Radius` 100.0 :`TraceChannel` "TraceTypeQuery1" :`DrawDebugType` "ForDuration")))