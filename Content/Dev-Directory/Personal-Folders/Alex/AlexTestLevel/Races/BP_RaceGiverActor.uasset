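; BP_RaceGiverActor is a race giver that offers a race to the pigeon character.
; On BeginPlay it loads its race details from DT_Races by name and sends them out through a dispatcher.
; Box overlap enables interaction, though end overlap never clears the flag.
; When allowed, Pickup shows the race widget, pauses the game and spawns a BP_RaceController carrying the details, checkpoints and a self-reference.
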(event `self.ReceiveBeginPlay`
  (`self.GetRaceDetails`))

(event `self.Box.OnComponentBeginOverlap`
  (params (OverlappedComponent :type "PrimitiveComponent Object Reference") (OtherActor :type "Actor Object Reference") (OtherComp :type "PrimitiveComponent Object Reference") (OtherBodyIndex :type Integer) (bFromSweep :type Boolean) (SweepResult :type "HitResult Structure (by ref)"))
  (cast `/Game/Dev-Directory/Personal-Folders/Alex/AlexTestLevel/PlayerCharacter/BP_PigeonCharacter_AB` OtherActor)
  (set `self.bCanInteract` true) ; Sets interactivity to true
  (`KismetSystemLibrary.PrintString` "Race Giver can be interacted with"))

(event `self.Box.OnComponentEndOverlap`
  (params (OverlappedComponent :type "PrimitiveComponent Object Reference") (OtherActor :type "Actor Object Reference") (OtherComp :type "PrimitiveComponent Object Reference") (OtherBodyIndex :type Integer))
  (cast `/Game/Dev-Directory/Personal-Folders/Alex/AlexTestLevel/PlayerCharacter/BP_PigeonCharacter_AB` OtherActor)
  (set `self.bCanInteract` (`self.bCanInteract`))
  (`KismetSystemLibrary.PrintString` "Racer interact range left"))

(event `/Game/Dev-Directory/Personal-Folders/Jayden/BPI_interact.Pickup`
  (bind _returnvalue (`GameplayStatics.GetPlayerController` 0))
  (bind (_racedetails_timeinseconds _racedetails_racename _racedetails_trinketreward) (break `/Game/Dev-Directory/Personal-Folders/Alex/AlexTestLevel/Races/S_RaceDetails` (`self.RaceDetails`)))
  (`self.EnableInput` _returnvalue)
  (if (`self.bCanInteract`)
    (bind _returnvalue_2 (`|CreateWidget` "/Game/Dev-Directory/Personal-Folders/Alex/AlexTestLevel/Races/WBP_RaceWidget.WBP_RaceWidget_C" _returnvalue _racedetails_timeinseconds _racedetails_trinketreward _racedetails_racename))
    (`UserWidget.AddToViewport` _returnvalue_2 0)
    (`GameplayStatics.SetGamePaused` true)
    (`|SpawnActorFromClass` "/Game/Dev-Directory/Personal-Folders/Alex/AlexTestLevel/Races/BP_RaceController.BP_RaceController_C" (`self.GetTransform`) "Undefined" "MultiplyWithRoot" null (`self.RaceDetails`) (`self.TotalCheckpoints`) self null)))

(fn `GetRaceDetails`
  (bind _returnvalue (`|GetDataTableRow` "/Game/Dev-Directory/Personal-Folders/Alex/AlexTestLevel/Races/DT_Races.DT_Races" (`self.RaceName`))
    (:`then`
      (bind _output_get (set `self.RaceDetails` (make `/Game/Dev-Directory/Personal-Folders/Alex/AlexTestLevel/Races/S_RaceDetails` (break `/Game/Dev-Directory/Personal-Folders/Alex/AlexTestLevel/Races/S_RaceDetails` _returnvalue) (`.RaceName_26_358054144019565B8170DC8169586067` (break `/Game/Dev-Directory/Personal-Folders/Alex/AlexTestLevel/Races/S_RaceDetails` _returnvalue)) (`.TrinketReward_25_F5A729914F5426F47069ADB3519088F0` (break `/Game/Dev-Directory/Personal-Folders/Alex/AlexTestLevel/Races/S_RaceDetails` _returnvalue)))))
      (`self.SendRaceDetails` (make `/Game/Dev-Directory/Personal-Folders/Alex/AlexTestLevel/Races/S_RaceDetails` (break `/Game/Dev-Directory/Personal-Folders/Alex/AlexTestLevel/Races/S_RaceDetails` _output_get) (`.RaceName_26_358054144019565B8170DC8169586067` (break `/Game/Dev-Directory/Personal-Folders/Alex/AlexTestLevel/Races/S_RaceDetails` _output_get)) (`.TrinketReward_25_F5A729914F5426F47069ADB3519088F0` (break `/Game/Dev-Directory/Personal-Folders/Alex/AlexTestLevel/Races/S_RaceDetails` _output_get)))))))

(fn `UserConstructionScript`)