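; BP_OldHud is a helper Blueprint with key bindings for the day cycle and the map.
; GetExtras caches the first 24HourCycle actor and the first BP_NewHud found in the level, then hides MapArrow.
; L adds to the cycle's Timer and K calls its SkipTime.
; M toggles the map on BP_NewHud and shows MapArrow only while that map is open.
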(event `GetExtras`
  ;[1 1 1] Get Extras
  (`self.Get24HourCycle`)
  (`self.GetHUDWidget`))

(event `Key|L`
  (params (Key :type "Key Structure"))
  (bind _24hourcycleref (`self.24HourCycleRef`))
  (:`Pressed`
    (set `/Game/Dev-Directory/Personal-Folders/Isaiah/Day-Night-Cycle/24-Hour-Cycle.Timer` (+ (`/Game/Dev-Directory/Personal-Folders/Isaiah/Day-Night-Cycle/24-Hour-Cycle.Timer` _24hourcycleref) 1.0) _24hourcycleref)))

(event `Get24HourCycle`
  ;[1 1 1] Get Extras
  (bind _outactors (`GameplayStatics.GetAllActorsOfClass` "/Game/Dev-Directory/Personal-Folders/Isaiah/Day-Night-Cycle/24-Hour-Cycle.24-Hour-Cycle_C"))
  (set `self.24HourCycleRef` (`|GetArrayItem` _outactors)))

(event `GetHUDWidget`
  ;[1 1 1] Get Extras
  (bind _outactors (`GameplayStatics.GetAllActorsOfClass` "/Game/Dev-Directory/Personal-Folders/Isaiah/Blueprints/BP_NewHud.BP_NewHud_C"))
  (set `self.NewHud` (`|GetArrayItem` _outactors))
  (`SceneComponent.SetVisibility` (`self.MapArrow`) false false))

(event `Key|K`
  (params (Key :type "Key Structure"))
  (:`Pressed`
    (`/Game/Dev-Directory/Personal-Folders/Isaiah/Day-Night-Cycle/24-Hour-Cycle.SkipTime` (`self.24HourCycleRef`))))

(event `Key|M`
  (params (Key :type "Key Structure"))
  (bind _newhud (`self.NewHud`))
  (:`Pressed`
    (`/Game/Dev-Directory/Personal-Folders/Isaiah/Blueprints/BP_NewHud.ToggleMap` _newhud)
    (if (`/Game/Dev-Directory/Personal-Folders/Isaiah/Blueprints/BP_NewHud.Is Map Open` _newhud)
      (`SceneComponent.SetVisibility` (`self.MapArrow`) true false)
      (else
        (`SceneComponent.SetVisibility` (`self.MapArrow`) false false)))))

(fn `UserConstructionScript`)