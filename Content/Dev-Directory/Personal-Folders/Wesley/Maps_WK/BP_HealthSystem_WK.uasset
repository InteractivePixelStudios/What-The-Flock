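; Blueprint health system that tracks current and maximum health, filling current health to max on BeginPlay.
; RestoreHealth and LoseHealth add or subtract an amount, clamping the result between zero and max health.
; IncreaseMaxHealth raises both max and current health by the same amount.
; E and R debug keys trigger a heal or damage for testing.
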(event EventBeginPlay
  ;[1 1 1] At start, set Current Health to Max Health
  (Variables|Default|SetHealthCurrent (Variables|Default|GetHealthMax)))

(event EventTick
  (params (DeltaSeconds :type Float%20%28single-precision%29)))

(event Input|KeyboardEvents|DebugKeyE
  (params (Key :type Key%20Structure :default "None") (ActionValue :type Input%20Action%20Value%20Structure))
  ;[1 1 1] Debug Stuff
  (:Pressed
    (CallFunction|RestoreHealth 2)))

(event Input|KeyboardEvents|DebugKeyR
  (params (Key :type Key%20Structure :default "None") (ActionValue :type Input%20Action%20Value%20Structure))
  ;[1 1 1] Debug Stuff
  (:Pressed
    (CallFunction|LoseHealth 1)))

(fn RestoreHealth
  (params (HealthRestored :type Integer))
  ;[1 1 1] Get Health restored and add it to current health, making sure it doesnt go above Max Health, and set the value to Current Health
  (Variables|Default|SetHealthCurrent (Math|Integer|Clamp(Integer) (+ HealthRestored (Variables|Default|GetHealthCurrent)) 0 (Variables|Default|GetHealthMax))) ; Set new Current Health
)

(fn LoseHealth
  (params (DamageTaken :type Integer))
  ;[1 1 1] Get Damage Taken and subtract it from current health, making sure it doesnt go below 0, and set the value to Current Health
  (Variables|Default|SetHealthCurrent (Math|Integer|Clamp(Integer) (- (Variables|Default|GetHealthCurrent) DamageTaken) 0 (Variables|Default|GetHealthMax))) ; Set new Current Health
)

(fn IncreaseMaxHealth
  (params (MaxHealthIncrease :type Integer))
  ;[1 1 1] When called, increases max health by the input value and restores that same value to current health
  (Variables|Default|SetHealthMax (+ (Variables|Default|GetHealthMax) MaxHealthIncrease)) ; Set Max Health to new value
  (Variables|Default|SetHealthCurrent (+ (Variables|Default|GetHealthCurrent) MaxHealthIncrease)) ; set new value to Current Health
)