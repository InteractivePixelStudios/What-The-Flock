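; BP_SubwayEntrance is a subway entrance trigger that shows the WBP_LevelTransition widget, apparently a work in progress in a test level folder.
; Box overlap begin and end set a ShouldShowWidget flag for any actor, which Tick checks every frame through ShowWidget.
; While set, each tick creates another widget and enables cursor and UI input.
; Otherwise it restores game-only input and removes WidgetRef, which this graph never assigns.
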(event `self.ReceiveTick`
  (params (DeltaSeconds :type "Float (single-precision)"))
  (`self.ShowWidget`))

(event `ShowWidget`
  (bind _returnvalue (`GameplayStatics.GetPlayerController` 0))
  (bind _returnvalue_2 (`GameplayStatics.GetPlayerController` 0))
  (if (`self.ShouldShowWidget`)
    (bind _returnvalue_3 (`|CreateWidget` "/Game/Dev-Directory/Personal-Folders/Alex/AlexTestLevel/LevelTransitions/WBP_LevelTransition.WBP_LevelTransition_C"))
    (`UserWidget.AddToViewport` _returnvalue_3 0)
    (`WidgetBlueprintLibrary.SetInputMode_GameAndUIEx` _returnvalue_2 _returnvalue_3 "DoNotLock" false)
    (set `PlayerController.bShowMouseCursor` true _returnvalue_2)
    (else
      (`WidgetBlueprintLibrary.SetInputMode_GameOnly` _returnvalue)
      (set `PlayerController.bShowMouseCursor` false _returnvalue)
      (`Widget.RemoveFromParent` (`self.WidgetRef`)))))

(event `self.Box.OnComponentBeginOverlap`
  (params (OverlappedComponent :type "PrimitiveComponent Object Reference") (OtherActor :type "Actor Object Reference") (OtherComp :type "PrimitiveComponent Object Reference") (OtherBodyIndex :type Integer) (bFromSweep :type Boolean) (SweepResult :type "HitResult Structure (by ref)"))
  (set `self.ShouldShowWidget` true))

(event `self.Box.OnComponentEndOverlap`
  (params (OverlappedComponent :type "PrimitiveComponent Object Reference") (OtherActor :type "Actor Object Reference") (OtherComp :type "PrimitiveComponent Object Reference") (OtherBodyIndex :type Integer))
  (set `self.ShouldShowWidget` false))

(fn `UserConstructionScript`)