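; Base dialogue component that opens and closes a conversation widget, switching input between UI and game and messaging its owner on close.
; Children presumably override the empty Dialogue function, which each progress step replays from the start.
; AddDialogue returns the stored choice for already-answered indices or displays the first unanswered line and options.
; Selections are saved in the DialogueProgress map, which can be rolled back, or cleared when switching tree index.
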(fn `AddDialogue`
  (params (Speaker :type Text) (Dialogue :type Text) (Options :type "Array of Text"))
  (returns (State :type "/Game/Dev-Directory/Personal-Folders/Jacob-Dialogue/Blueprints/Enum_DialogueState Enum") (OptionIndex :type Integer))
  (bind (_value _returnvalue) (`BlueprintMapLibrary.Map_Find` (`self.DialogueProgress`) (`self.DialogueIndex`)))
  (`/Engine/EditorBlueprintResources/StandardMacros.IncrementInt` (`self.DialogueIndex`)
    (:`  `
      (if _returnvalue
        (return "NewEnumerator0" _value)
        (else
          ;[1 1 1] Updates the dialogue text
          (`/Game/UI/W_Dialogue.UpdateDialogueText` (`self.DialogueWidget`) (`self.DialogueIndex`) (`local.Speaker`) (`local.Dialogue`) (`local.Options`))
          (return "NewEnumerator1" 0))))))

(fn `ClearDialogueProgress`
  ;[1 1 1] Sets dialogue progress back to the beginning
  (`BlueprintMapLibrary.Map_Clear` (`self.DialogueProgress`)))

(fn `CloseConversation`
  (bind _returnvalue (`GameplayStatics.GetPlayerController` 0))
  ;[1 1 1] Deletes the dialogue widget and closes the conversation.
  (`Widget.RemoveFromParent` (`self.DialogueWidget`))
  (message `/Game/Dev-Directory/Personal-Folders/Jacob-Dialogue/Blueprints/BPI_Interactable.ConversationClosed` (`self.GetOwner`))
  (`WidgetBlueprintLibrary.SetInputMode_GameOnly` _returnvalue)
  (set `PlayerController.bShowMouseCursor` false _returnvalue))

(fn `Dialogue`)

(fn `OpenConversation`
  (bind _returnvalue (`GameplayStatics.GetPlayerController` 0))
  ;[1 1 1] Creates a new dialogue widget and overlay on the screen
  (bind _returnvalue_2 (`|CreateWidget` "/Game/UI/W_Dialogue.W_Dialogue_C" null self))
  (bind _output_get (set `self.DialogueWidget` _returnvalue_2))
  (`UserWidget.AddToViewport` _output_get 0)
  ;[1 1 1] Enable UI
  (`WidgetBlueprintLibrary.SetInputMode_UIOnlyEx` _returnvalue _output_get)
  (set `PlayerController.bShowMouseCursor` true _returnvalue)
  ;[1 1 1] Calls the progress dialogue function
  (`self.ProgressDialogue`))

(fn `ProgressDialogue`
  ;[1 1 1] Resetting the dialogue index per new dialogue options
  (set `self.DialogueIndex` -1)
  (`self.Dialogue`)
  (`KismetSystemLibrary.PrintString` "Progressing Dialogue"))

(fn `RemoveDialogueProgress`
  (params (ProgressSteps :type Integer))
  ;[1 1 1] Goes to the end of the dialogue index and removes progress from the index to see the previous dialogue.
  (for _index (range (+ ProgressSteps 1))
    (`BlueprintMapLibrary.Map_Remove` (`self.DialogueProgress`) (- (`self.DialogueIndex`) _index))))

(fn `SetDialogueTreeIndex`
  (params (DialogueTreeIndex :type Integer))
  ;[1 1 1] Sets the dialogue tree index and then calls to clear dialogue progress
  (set `self.DialogueTreeIndex` DialogueTreeIndex)
  (`self.ClearDialogueProgress`))

(fn `UpdateSelectedOption`
  (params (ProgressIndex :type "Integer (by ref)") (OptionIndex :type "Integer (by ref)"))
  ;[1 1 1] Increase dialogue progress when option is selected
  (`BlueprintMapLibrary.Map_Add` (`self.DialogueProgress`) ProgressIndex OptionIndex)
  (`self.ProgressDialogue`))