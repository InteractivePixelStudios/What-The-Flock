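; Temporary Blueprint, named as logic to add back into the pigeon Blueprint, that lets the player look at and interact with quest actors.
; Each tick, InteractionTrace casts a short camera-forward line trace, stores any hit implementing BPI_QuestInteractionInterface and sends it a look-at message.
; When IA_Pickup completes, it messages the stored actor and broadcasts the returned value as an objective ID.
; An unconnected copy of the trace remains in the EventGraph.
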(event `self.ReceiveTick`
  (params (DeltaSeconds :type "Float (single-precision)"))
  ;[1 1 1] Event Tick
  (`self.InteractionTrace`))

(event `EnhancedInput|/Game/Dev-Directory/Personal-Folders/Alex/AlexTestLevel/EnhancedInput/IA_Pickup`
  (params (ActionValue :type Boolean) (ElapsedSeconds :type "Float (double-precision)") (TriggeredSeconds :type "Float (double-precision)") (InputAction :type "InputAction Object Reference" :default "/Game/Dev-Directory/Personal-Folders/Alex/AlexTestLevel/EnhancedInput/IA_Pickup.IA_Pickup"))
  ;[1 1 1] Event Tick
  (:`Completed`
    (bind _lookatquestactor (`self.lookAtQuestActor`)
      (:`then`
        (bind _objectiveid (message `/Game/Dev-Directory/Personal-Folders/Alex/AlexTestLevel/QuestSystem/BPI_QuestInteractionInterface.InteractWithNPC` _lookatquestactor))
        (`self.OnObjectiveIDCalled` (`KismetStringLibrary.Conv_StringToName` _objectiveid)))
      (:`else`))))

(fn `InteractionTrace`
  (bind _returnvalue (`GameplayStatics.GetPlayerCameraManager` 0))
  (bind _returnvalue_2 (`self.K2_GetActorLocation` _returnvalue))
  ;[1 1 1] Line trace by actor location + (forwardvector*500)
  (bind (_outhit _returnvalue_3) (`KismetSystemLibrary.LineTraceSingle` _returnvalue_2 (+ _returnvalue_2 (* (`self.GetActorForwardVector` _returnvalue) 500.0)) "TraceTypeQuery2"))
  ;[1 1 1] On hit check if hit object has the quest interaction interface
  (if _returnvalue_3
    (bind (_bblockinghit _binitialoverlap _time _distance _location _impactpoint _normal _impactnormal _physmat _hitactor) (`GameplayStatics.BreakHitResult` _outhit))
    ;[1 1 1] Sets the quest giver
    (if (`KismetSystemLibrary.DoesImplementInterface` _hitactor "/Game/Dev-Directory/Personal-Folders/Alex/AlexTestLevel/QuestSystem/BPI_QuestInteractionInterface.BPI_QuestInteractionInterface_C")
      (bind _output_get (set `self.lookAtQuestActor` _hitactor))
      (message `/Game/Dev-Directory/Personal-Folders/Alex/AlexTestLevel/QuestSystem/BPI_QuestInteractionInterface.LookAtNPC` _output_get)
      (else
        (set `self.lookAtQuestActor` null)))
    (else
      (set `self.lookAtQuestActor` null))))

(fn `UserConstructionScript`)