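; BP_CustomPawn is a pawn that mirrors player stats, apparently for HUD display.
; On BeginPlay it copies Health, Stamina, Dooky and EXP from BPPlayerStats into matching Listener variables.
; The UpdateHUD event re-runs the same copy, so the values refresh only when that event fires, with no Tick or binding in the graph.
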(event `self.ReceiveBeginPlay`
  (set `self.HealthListener` (`/Game/Isaiah/Blueprints/BP_PlayerStats.Health` (`self.BP_PlayerStats`)) :!label _label)
  (set `self.StaminaListener` (`/Game/Isaiah/Blueprints/BP_PlayerStats.Stamina` (`self.BP_PlayerStats`)))
  (set `self.DookyListener` (`/Game/Isaiah/Blueprints/BP_PlayerStats.Dooky` (`self.BP_PlayerStats`)))
  (set `self.EXPListener` (`/Game/Isaiah/Blueprints/BP_PlayerStats.EXP` (`self.BP_PlayerStats`))))

(event `UpdateHUD`
  (goto _label))

(fn `UserConstructionScript`)