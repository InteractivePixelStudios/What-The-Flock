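; BP_ArrowPointer is a helper actor that floats above an owner and points an arrow at a target actor.
; An external caller assigns the owner and target through SetOwnerAndTarget and can retarget it with SetNewTarget.
; Each Tick, while the target is valid, it moves to a fixed offset from the owner and rotates ArrowBody toward the target with FindLookAtRotation.
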(event `self.ReceiveTick`
  (params (DeltaSeconds :type "Float (single-precision)"))
  ;[0.1059 0.1059 0.1059 0.7216] Check for valid target to follow
  (`/Engine/EditorBlueprintResources/StandardMacros.IsValid` (`self.TargetRef`)
    (:`Is Valid`
      ;[0.2623 0.552 1] Set arrow location to above owner
      (`self.K2_SetActorLocation` self (+ (`self.K2_GetActorLocation` (`self.OwnerRef`)) (0.0 5.0 10.0)) false false)
      ;[0.2623 0.552 1] Set the arrows rotation to point to target
      (`SceneComponent.K2_SetWorldRotation` (`self.ArrowBody`) (`KismetMathLibrary.FindLookAtRotation` (`self.K2_GetActorLocation` self) (`self.K2_GetActorLocation` (`self.TargetRef`))) false false))))

(fn `SetNewTarget`
  (params (`New Target` :type "Actor Object Reference"))
  ;[0.2623 0.552 1] Used to set new target for arrow to point at
  (set `self.TargetRef` `New Target`))

(fn `SetOwnerAndTarget`
  (params (Target :type "Actor Object Reference") (Owner :type "Pawn Object Reference"))
  ;[0.2623 0.552 1] Sets starting variables after creation
  (set `self.TargetRef` Target)
  (set `self.OwnerRef` Owner))

(fn `UserConstructionScript`)