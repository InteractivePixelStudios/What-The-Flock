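; Merchant table that displays items for the pigeon player and opens a shop widget.
; On BeginPlay it spawns cuttlebone and cricket pickups at four slots, with their sphere collision disabled.
; Four overlap boxes toggle CanInteract, letting Pickup show the widget, pause the game and switch to UI input.
; BuyItem, fired by event or debug key, deactivates or destroys the overlapped box's slot component, without any trinket cost check.
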(event OnComponentBeginOverlap(Box3)
  (params (OverlappedComponent :type Primitive%20Component%20Object%20Reference) (OtherActor :type Actor%20Object%20Reference) (OtherComp :type Primitive%20Component%20Object%20Reference) (OtherBodyIndex :type Integer) (bFromSweep :type Boolean) (SweepResult :type Hit%20Result%20Structure%20%28by%20ref%29))
  (Utilities|Casting|CastToBP_PigeonCharacter_AB OtherActor)
  (Variables|Default|SetbCanInteract true) ; Sets interactivity to true
  (Development|PrintString "Merchant can be interacted with"))

(event OnComponentBeginOverlap(Box1)
  (params (OverlappedComponent :type Primitive%20Component%20Object%20Reference) (OtherActor :type Actor%20Object%20Reference) (OtherComp :type Primitive%20Component%20Object%20Reference) (OtherBodyIndex :type Integer) (bFromSweep :type Boolean) (SweepResult :type Hit%20Result%20Structure%20%28by%20ref%29))
  (Utilities|Casting|CastToBP_PigeonCharacter_AB OtherActor)
  (Variables|Default|SetbCanInteract true) ; Sets interactivity to true
  (Development|PrintString "Merchant can be interacted with"))

(event OnComponentEndOverlap(Box1)
  (params (OverlappedComponent :type Primitive%20Component%20Object%20Reference) (OtherActor :type Actor%20Object%20Reference) (OtherComp :type Primitive%20Component%20Object%20Reference) (OtherBodyIndex :type Integer))
  (Utilities|Casting|CastToBP_PigeonCharacter_AB OtherActor)
  (Variables|Default|SetbCanInteract false)
  (Development|PrintString "Merchant interact range left"))

(event OnComponentBeginOverlap(Box)
  (params (OverlappedComponent :type Primitive%20Component%20Object%20Reference) (OtherActor :type Actor%20Object%20Reference) (OtherComp :type Primitive%20Component%20Object%20Reference) (OtherBodyIndex :type Integer) (bFromSweep :type Boolean) (SweepResult :type Hit%20Result%20Structure%20%28by%20ref%29))
  (Utilities|Casting|CastToBP_PigeonCharacter_AB OtherActor)
  (Variables|Default|SetbCanInteract true) ; Sets interactivity to true
  (Development|PrintString "Merchant can be interacted with"))

(event OnComponentEndOverlap(Box)
  (params (OverlappedComponent :type Primitive%20Component%20Object%20Reference) (OtherActor :type Actor%20Object%20Reference) (OtherComp :type Primitive%20Component%20Object%20Reference) (OtherBodyIndex :type Integer))
  (Utilities|Casting|CastToBP_PigeonCharacter_AB OtherActor)
  (Variables|Default|SetbCanInteract false)
  (Development|PrintString "Merchant interact range left"))

(event OnComponentBeginOverlap(Box2)
  (params (OverlappedComponent :type Primitive%20Component%20Object%20Reference) (OtherActor :type Actor%20Object%20Reference) (OtherComp :type Primitive%20Component%20Object%20Reference) (OtherBodyIndex :type Integer) (bFromSweep :type Boolean) (SweepResult :type Hit%20Result%20Structure%20%28by%20ref%29))
  (Utilities|Casting|CastToBP_PigeonCharacter_AB OtherActor)
  (Variables|Default|SetbCanInteract true) ; Sets interactivity to true
  (Development|PrintString "Merchant can be interacted with"))

(event OnComponentEndOverlap(Box2)
  (params (OverlappedComponent :type Primitive%20Component%20Object%20Reference) (OtherActor :type Actor%20Object%20Reference) (OtherComp :type Primitive%20Component%20Object%20Reference) (OtherBodyIndex :type Integer))
  (Utilities|Casting|CastToBP_PigeonCharacter_AB OtherActor)
  (Variables|Default|SetbCanInteract false)
  (Development|PrintString "Merchant interact range left"))

(event OnComponentEndOverlap(Box3)
  (params (OverlappedComponent :type Primitive%20Component%20Object%20Reference) (OtherActor :type Actor%20Object%20Reference) (OtherComp :type Primitive%20Component%20Object%20Reference) (OtherBodyIndex :type Integer))
  (Utilities|Casting|CastToBP_PigeonCharacter_AB OtherActor)
  (Variables|Default|SetbCanInteract false)
  (Development|PrintString "Merchant interact range left"))

(event Custom|BuyingItem_Event
  (CallFunction|BuyItem))

(event EventBeginPlay
  (CallFunction|PopulateTable)
  (CallFunction|GetPlayerTrinkets))

(event Collision|EventActorBeginOverlap
  (params (OtherActor :type Actor%20Object%20Reference)))

(event EventTick
  (params (DeltaSeconds :type Float%20%28single-precision%29)))

(event EventPickup
  (bind _returnvalue (Game|GetPlayerController 0))
  (Input|EnableInput _returnvalue)
  (if (Variables|Default|GetbCanInteract)
    (bind _returnvalue_2 (UserInterface|CreateWidget "/Game/Dev-Directory/Personal-Folders/Alex/AlexTestLevel/InteractWithMerchant/WBP_MerchantWidget.WBP_MerchantWidget_C" _returnvalue))
    (UserInterface|Viewport|AddtoViewport _returnvalue_2 0)
    (Game|SetGamePaused true)
    (Input|SetInputModeUIOnly _returnvalue (Variables|Default|GetMechantWidgetRef) "DoNotLock" false)
    (Variables|/Script/Engine.PlayerController|SetbShowMouseCursor _returnvalue true)))

(event Input|KeyboardEvents|DebugKeyR
  (params (Key :type Key%20Structure :default "None") (ActionValue :type Input%20Action%20Value%20Structure))
  (:Pressed
    (CallFunction|BuyItem)))

(fn ConstructionScript)

(fn PopulateTable
  (bind _returnvalue (Game|SpawnActorfromClass "/Game/Dev-Directory/Personal-Folders/Alex/AlexTestLevel/RareConsumables/BP_Cuttlebone.BP_Cuttlebone_C" (Transformation|GetSocketTransform (Variables|Default|GetItemSlot1) "None" "RTS_World") "Undefined" "OverrideRootScale" 0 0))
  (Collision|SetCollisionEnabled (Variables|/Game/Dev-Directory/Personal-Folders/Alex/AlexTestLevel/RareConsumables/BP_Cuttlebone.BP_Cuttlebone_C|GetSphere1 _returnvalue) "NoCollision")
  (AddComponent|AddChildActorComponent _returnvalue false)
  (bind _returnvalue_2 (Game|SpawnActorfromClass "/Game/Dev-Directory/Personal-Folders/Alex/AlexTestLevel/RareConsumables/BP_Crickets.BP_Crickets_C" (Transformation|GetSocketTransform (Variables|Default|GetItemSlot2) "None" "RTS_World") "Undefined" "OverrideRootScale" 0 0))
  (Collision|SetCollisionEnabled (Variables|/Game/Dev-Directory/Personal-Folders/Alex/AlexTestLevel/RareConsumables/BP_Crickets.BP_Crickets_C|GetSphere1 _returnvalue_2) "NoCollision")
  (AddComponent|AddChildActorComponent _returnvalue_2 false)
  (bind _returnvalue_3 (Game|SpawnActorfromClass "/Game/Dev-Directory/Personal-Folders/Alex/AlexTestLevel/RareConsumables/BP_Cuttlebone.BP_Cuttlebone_C" (Transformation|GetSocketTransform (Variables|Default|GetItemSlot3) "None" "RTS_World") "Undefined" "OverrideRootScale" 0 0))
  (Collision|SetCollisionEnabled (Variables|/Game/Dev-Directory/Personal-Folders/Alex/AlexTestLevel/RareConsumables/BP_Cuttlebone.BP_Cuttlebone_C|GetSphere1 _returnvalue_3) "NoCollision")
  (AddComponent|AddChildActorComponent _returnvalue_3 false)
  (bind _returnvalue_4 (Game|SpawnActorfromClass "/Game/Dev-Directory/Personal-Folders/Alex/AlexTestLevel/RareConsumables/BP_Cuttlebone.BP_Cuttlebone_C" (Transformation|GetSocketTransform (Variables|Default|GetItemSlot4) "None" "RTS_World") "Undefined" "OverrideRootScale" 0 0))
  (Collision|SetCollisionEnabled (Variables|/Game/Dev-Directory/Personal-Folders/Alex/AlexTestLevel/RareConsumables/BP_Cuttlebone.BP_Cuttlebone_C|GetSphere1 _returnvalue_4) "NoCollision")
  (AddComponent|AddChildActorComponent _returnvalue_4 false))

(fn GetPlayerTrinkets
  (Variables|Default|GetPlayerRef
    (:then
      (Variables|Default|SetPlayerCurrentTrinkets 0))
    (:else)))

(fn BuyItem
  (bind _playerref (Variables|Default|GetPlayerRef)
    (:then
      (if (Class|PrimitiveComponent|IsOverlappingComponent (Variables|Default|GetBox) (Variables|/Script/Engine.Character|GetMesh _playerref))
        (Components|Activation|Deactivate (Variables|Default|GetItemSlot1))
        (elif (Class|PrimitiveComponent|IsOverlappingComponent (Variables|Default|GetBox1) (Variables|/Script/Engine.Character|GetMesh _playerref))
          (Components|Activation|Deactivate (Variables|Default|GetItemSlot2))
          (elif (Class|PrimitiveComponent|IsOverlappingComponent (Variables|Default|GetBox2) (Variables|/Script/Engine.Character|GetMesh _playerref))
            (Components|Activation|Deactivate (Variables|Default|GetItemSlot3))
            (elif (Class|PrimitiveComponent|IsOverlappingComponent (Variables|Default|GetBox3) (Variables|/Script/Engine.Character|GetMesh _playerref))
              (Components|DestroyComponent (Variables|Default|GetItemSlot4)))))))
    (:else)))