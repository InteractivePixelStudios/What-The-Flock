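; Player controller for the respawn system, which opens a respawn map and teleports the player to the selected respawn point.
; The pause-respawn input lazily creates the map and pick widgets, shows the map, switches to UI input and moves the view to BP_RespawnCamera.
; RespawnPlayer moves the pawn slightly above BP_RespawnManager's current point, removes both widgets and restores game input and camera.
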(event `self.ReceiveBeginPlay`
  (bind _returnvalue (`GameplayStatics.GetPlayerController` 0))
  (`WidgetBlueprintLibrary.SetInputMode_GameOnly` _returnvalue)
  (message `EnhancedInputSubsystemInterface.AddMappingContext` (pcsubsystem `EnhancedInputLocalPlayerSubsystem` _returnvalue) "/Game/Dev-Directory/Personal-Folders/Amelia/RespawnSystem/InputActions/IMC_Respawn_Testing.IMC_Respawn_Testing" 0 (struct))
  (bind _returnvalue_2 (`GameplayStatics.GetActorOfClass` "/Game/Dev-Directory/Personal-Folders/Amelia/RespawnSystem/BP_RespawnCamera.BP_RespawnCamera_C"))
  (set `self.RespawnCamera` _returnvalue_2))

(event `RespawnPlayer`
  (bind _returnvalue (`GameplayStatics.GetPlayerController` 0))
  (bind _returnvalue_2 (`GameplayStatics.GetActorOfClass` "/Game/Dev-Directory/Personal-Folders/Amelia/RespawnSystem/RespawnSystem/BP_RespawnManager.BP_RespawnManager_C"))
  ;[0.231 0.1121 0.5521] Teleports player to selected respawn point
  (bind _newparam (`/Game/Dev-Directory/Personal-Folders/Amelia/RespawnSystem/RespawnSystem/BP_RespawnManager.GetCurrentRespawnPoint` _returnvalue_2))
  (`self.K2_SetActorLocation` (`GameplayStatics.GetPlayerPawn` 0) (`KismetMathLibrary.MakeVector` (.x (`self.K2_GetActorLocation` _newparam)) (.y (`self.K2_GetActorLocation` _newparam)) (+ (.z (`self.K2_GetActorLocation` _newparam)) 50.0)) false false)
  (`Widget.RemoveFromParent` (`self.Debug Reference`))
  (`Widget.RemoveFromParent` (`self.Pause Reference`))
  (set `self.IsRespawning` false)
  ;[1 1 1] Returns camera and control to the player
  (set `PlayerController.bShowMouseCursor` false _returnvalue)
  (`WidgetBlueprintLibrary.SetInputMode_GameOnly` _returnvalue)
  (`self.EnableInput` _returnvalue)
  (`self.SetViewTargetWithBlend` (`ActorComponent.GetOwner` (`Actor.RootComponent` (`self.PlayerCameraManager`)))))

(event `EnhancedInput|/Game/Dev-Directory/Personal-Folders/Amelia/RespawnSystem/InputActions/IA_PauseMenu_Respawn`
  (params (ActionValue :type Boolean) (ElapsedSeconds :type "Float (double-precision)") (TriggeredSeconds :type "Float (double-precision)") (InputAction :type "InputAction Object Reference" :default "/Game/Dev-Directory/Personal-Folders/Amelia/RespawnSystem/InputActions/IA_PauseMenu_Respawn.IA_PauseMenu_Respawn"))
  (bind _returnvalue (`GameplayStatics.GetPlayerController` 0))
  (bind _pause_reference (`self.Pause Reference`))
  (:`Started`
    (`/Engine/EditorBlueprintResources/StandardMacros.IsValid` (`self.Pause Reference`)
      (:`Is Valid`
        _)
      (:`Is Not Valid`
        ;[1 1 1] If widget doesn't exist, make one
        (bind _returnvalue_2 (`|CreateWidget` "/Game/Dev-Directory/Personal-Folders/Amelia/RespawnSystem/UW_RespawnMap.UW_RespawnMap_C"))
        (set `self.Pause Reference` _returnvalue_2)
        (bind _returnvalue_3 (`|CreateWidget` "/Game/Dev-Directory/Personal-Folders/Amelia/RespawnSystem/UW_PickRespawn.UW_PickRespawn_C"))
        (set `self.Debug Reference` _returnvalue_3)))
    (if (not (`self.IsRespawning`))
      (`UserWidget.AddToViewport` _pause_reference 0)
      (set `self.IsRespawning` false)
      ;[1 1 1] Takes away player control and enters respawn UI
      (set `PlayerController.bShowMouseCursor` true _returnvalue)
      (`self.DisableInput` _returnvalue)
      (`WidgetBlueprintLibrary.SetInputMode_GameAndUIEx` _returnvalue _pause_reference)
      (`self.SetViewTargetWithBlend` (`self.RespawnCamera`)))))

(fn `UserConstructionScript`)