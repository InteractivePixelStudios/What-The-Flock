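; Large pigeon nest that stays hidden while inactive, shimmers into view when the pigeon comes near, and opens a menu once active.
; BeginPlay picks the nest or shimmer material from Active, and the visibility radius shows or hides inactive nests.
; The interact radius sets CanInteract on active nests, letting Pickup open the nest menu, pause and switch to UI input.
; Material and visibility functions extend parent versions, with SwapMaterials alternating via FlipFlop.
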(event `self.ReceiveBeginPlay`
  (bind _nest (`self.Nest`))
  ;[1 1 1] If the nest is already active, swap to proper material, otherwise set to the shimmer material
  (if (`self.Active`)
    (`PrimitiveComponent.SetMaterial` _nest 0 (`self.NestMaterial`)) ; Set nest to Nest Material
    (else
      (`PrimitiveComponent.SetMaterial` _nest 0 (`self.ShimmerMaterial`)) ; Set nest to Shimmer Material
      (`self.MakeInvisible`) ; Make invisible on start
    )))

(event `self.NestVisibilityRadius.OnComponentBeginOverlap`
  (params (OverlappedComponent :type "PrimitiveComponent Object Reference") (OtherActor :type "Actor Object Reference") (OtherComp :type "PrimitiveComponent Object Reference") (OtherBodyIndex :type Integer) (bFromSweep :type Boolean) (SweepResult :type "HitResult Structure (by ref)"))
  ;[1 1 1] Once player enters collision area, if not active, make nest visible
  (cast `/Game/Dev-Directory/Personal-Folders/Alex/AlexTestLevel/PlayerCharacter/BP_PigeonCharacter_AB` OtherActor)
  (if (not (`self.Active`))
    (`self.MakeVisible`)))

(event `self.NestVisibilityRadius.OnComponentEndOverlap`
  (params (OverlappedComponent :type "PrimitiveComponent Object Reference") (OtherActor :type "Actor Object Reference") (OtherComp :type "PrimitiveComponent Object Reference") (OtherBodyIndex :type Integer))
  ;[1 1 1] Once player leaves collision area, make non-active nest invisible
  (cast `/Game/Dev-Directory/Personal-Folders/Alex/AlexTestLevel/PlayerCharacter/BP_PigeonCharacter_AB` OtherActor)
  (if (not (`self.Active`))
    (`self.MakeInvisible`)))

(event `self.NestInteractRadius.OnComponentBeginOverlap`
  (params (OverlappedComponent :type "PrimitiveComponent Object Reference") (OtherActor :type "Actor Object Reference") (OtherComp :type "PrimitiveComponent Object Reference") (OtherBodyIndex :type Integer) (bFromSweep :type Boolean) (SweepResult :type "HitResult Structure (by ref)"))
  ;[1 1 1] On Enter Interactive range
  (cast `/Game/Dev-Directory/Personal-Folders/Alex/AlexTestLevel/PlayerCharacter/BP_PigeonCharacter_AB` OtherActor)
  (if (`self.Active`)
    (set `self.bCanInteract` true) ; Sets interactivity to true
    (`KismetSystemLibrary.PrintString` "Nest can be interacted with")))

(event `self.NestInteractRadius.OnComponentEndOverlap`
  (params (OverlappedComponent :type "PrimitiveComponent Object Reference") (OtherActor :type "Actor Object Reference") (OtherComp :type "PrimitiveComponent Object Reference") (OtherBodyIndex :type Integer))
  ;[1 1 1] On Leave Interactive range
  (cast `/Game/Dev-Directory/Personal-Folders/Alex/AlexTestLevel/PlayerCharacter/BP_PigeonCharacter_AB` OtherActor)
  (if (`self.Active`)
    (set `self.bCanInteract` false)
    (`KismetSystemLibrary.PrintString` "Nest interact range left")))

(event `/Game/Dev-Directory/Personal-Folders/Jayden/BPI_interact.Pickup`
  (bind _returnvalue (`GameplayStatics.GetPlayerController` 0))
  ;[1 1 1] Interactive mode
  (`self.EnableInput` _returnvalue)
  (if (`self.bCanInteract`)
    (bind _returnvalue_2 (`|CreateWidget` "/Game/Dev-Directory/Personal-Folders/Jacob-EXP/Nest-Materials/BP_NestMenu.BP_NestMenu_C" _returnvalue))
    (`UserWidget.AddToViewport` _returnvalue_2 0)
    (`GameplayStatics.SetGamePaused` true)
    (`WidgetBlueprintLibrary.SetInputMode_UIOnlyEx` _returnvalue null)
    (set `PlayerController.bShowMouseCursor` true _returnvalue)))

(fn `MakeInvisible`
  ;[1 1 1] Set nest to not visible
  (`parent.MakeInvisible`)
  (`SceneComponent.SetVisibility` (`self.Nest`) false false))

(fn `MakeVisible`
  ;[1 1 1] Set nest to be visible
  (`parent.MakeVisible`)
  (`SceneComponent.SetVisibility` (`self.Nest`) true false))

(fn `SwapMaterials`
  ;[1 1 1] Flip through Shimmer/Nest materials as called
  (`parent.SwapMaterials`)
  (`/Engine/EditorBlueprintResources/StandardMacros.FlipFlop`
    (:`A`
      ;[1 1 1] First call sets material to Nest Material
      (`PrimitiveComponent.SetMaterial` (`self.Nest`) 0 (`self.NestMaterial`)))
    (:`B`
      ;[1 1 1] Second Call will reset nest back to Shimmer Material
      (`PrimitiveComponent.SetMaterial` (`self.Nest`) 0 (`self.ShimmerMaterial`)))))

(fn `UserConstructionScript`
  (`parent.UserConstructionScript`))