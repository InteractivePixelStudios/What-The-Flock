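; BP_AudioWizard is a level audio manager that runs world ambience and gives enemy AI cars their sound.
; On BeginPlay it plays a looping suburb ambience, then spawns and attaches a BP_CarAudioFromLocation to each BP_AICarEnemy present.
; SetCarAudio assigns a placeholder sound to all those emitters, re-running after every spawn.
; Tick re-applies a one-second ambience volume fade from master times ambience volume; the CarAudio function is an empty stub.
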(event `Ambience`
  ;[1 1 1] World Ambience
  (`AudioComponent.Play` (`self.Ambience1`) 0.0))

(event `GetAllCars`
  ;[1 1 1] Car Audio
  (bind _outactors (`GameplayStatics.GetAllActorsOfClass` "/Game/Dev-Directory/Personal-Folders/Alex/AlexTestLevel/TrafficSystem/BP_AICarEnemy.BP_AICarEnemy_C"))
  (for _array_element _outactors
    (bind _returnvalue (`|SpawnActorFromClass` "/Game/Dev-Directory/Personal-Folders/Isaiah/Audio/BP_CarAudioFromLocation.BP_CarAudioFromLocation_C" (`KismetMathLibrary.Conv_VectorToTransform` (`self.K2_GetActorLocation` _array_element)) "Undefined" "MultiplyWithRoot" _array_element null))
    (`self.K2_AttachToActor` _returnvalue _array_element "None" "SnapToTarget" "SnapToTarget" "KeepWorld" true)
    (`self.SetCarAudio`)))

(event `SetCarAudio`
  ;[1 1 1] Car Audio
  (bind _outactors (`GameplayStatics.GetAllActorsOfClass` "/Game/Dev-Directory/Personal-Folders/Isaiah/Audio/BP_CarAudioFromLocation.BP_CarAudioFromLocation_C"))
  (for _array_element _outactors
    (`AudioComponent.SetSound` (`/Game/Dev-Directory/Personal-Folders/Isaiah/Audio/BP_CarAudioFromLocation.Audio` _array_element) "/Game/Dev-Directory/Personal-Folders/Isaiah/Audio/Cars/CarAudioPlaceholder.CarAudioPlaceholder")))

(event `self.ReceiveTick`
  (params (DeltaSeconds :type "Float (single-precision)"))
  (`self.AdjustVolume`))

(event `self.ReceiveBeginPlay`
  (`AudioComponent.SetSound` (`self.Ambience1`) "/Game/Dev-Directory/Personal-Folders/Isaiah/Audio/Ambience/Suburb_Loop_B.Suburb_Loop_B")
  (`self.Ambience`)
  (`self.GetAllCars`))

(event `AdjustVolume`
  (`AudioComponent.AdjustVolume` (`self.Ambience1`) 1.0 (* (`self.MasterVolume`) (`self.AmbienceVolume`)) "Linear"))

(fn `CarAudio`)

(fn `UserConstructionScript`)