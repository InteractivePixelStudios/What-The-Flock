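; Player flight controller that lets the character fly after a quick double jump, driving the player character's movement component.
; While flying, Tick applies forward glide and downward gravity forces along the control yaw.
; Flap input spends stamina for an upward impulse, and move input adds forward movement and yaw turning.
; A box overlap below the character detects WorldStatic ground and switches movement back to Falling.
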(event `self.ReceiveBeginPlay`
  ;[1 1 1] Set Base Variables
  (`self.GetParentCharacterController`)
  (set `self.stamina` (`self.MAX_STAMINA`)))

(event `self.ReceiveTick`
  (params (DeltaSeconds :type "Float (single-precision)"))
  ;[1 1 1] If flying apply gravity and forward glide while checking if the player hit the ground
  (if (`self.isFlying`)
    (`self.FallAndGlide`)
    (bind _groundcheck (`self.GroundCheck`))
    ;[1 1 1] When player hits the ground set flying to false and make the character fall to the ground
    (if _groundcheck
      (set `self.isFlying` false)
      (`CharacterMovementComponent.SetMovementMode` (`self.characterMovementComponent`) "MOVE_Falling" 0))))

(event `EnhancedInput|/Game/Dev-Directory/Personal-Folders/Sebastian/InputActions/IA_FlapUp`
  (params (ActionValue :type Boolean) (ElapsedSeconds :type "Float (double-precision)") (TriggeredSeconds :type "Float (double-precision)") (InputAction :type "InputAction Object Reference" :default "/Game/Dev-Directory/Personal-Folders/Sebastian/InputActions/IA_FlapUp.IA_FlapUp"))
  (bind _stamina (`self.stamina`))
  (:`Started`
    (if (`self.isFlying`)
      ;[1 1 1] Check if player has the stamina to Flap wings
      (if (> _stamina 1.0)
        ;[1 1 1] Decrement Stamina and add upward force to the player
        (bind _result (`/Engine/EditorBlueprintResources/StandardMacros.DecrementFloat` _stamina)
          (:`  `
            (set `self.stamina` _result)
            (`CharacterMovementComponent.AddImpulse` (`self.characterMovementComponent`) (`KismetMathLibrary.MakeVector` 0.0 0.0 (`self.flightFlapUpForce`)) false)))))))

(event `EnhancedInput|/Game/Dev-Directory/Personal-Folders/Alex/AlexTestLevel/EnhancedInput/IA_Jump`
  (params (ActionValue :type Boolean) (ElapsedSeconds :type "Float (double-precision)") (TriggeredSeconds :type "Float (double-precision)") (InputAction :type "InputAction Object Reference" :default "/Game/Dev-Directory/Personal-Folders/Alex/AlexTestLevel/EnhancedInput/IA_Jump.IA_Jump"))
  (:`Started`
    ;[1 1 1] If not flying increment jump to attempt to fly
    (if (not (`self.isFlying`))
      (bind _result (`/Engine/EditorBlueprintResources/StandardMacros.IncrementInt` (`self.jumpCount`))
        (:`  `
          ;[1 1 1] If jumped twice then set player to flying
          (if (== _result 2)
            (`CharacterMovementComponent.SetMovementMode` (`self.characterMovementComponent`) "MOVE_Flying" 0)
            (set `self.isFlying` true)
            (else
              ;[1 1 1] Else reset jump count after half second
              (`KismetSystemLibrary.RetriggerableDelay` 0.5)
              (set `self.jumpCount` 0))))))))

(event `EnhancedInput|/Game/Dev-Directory/Personal-Folders/Sebastian/InputActions/IA_FlyMove`
  (params (ActionValue :type "Vector2D Structure") (ElapsedSeconds :type "Float (double-precision)") (TriggeredSeconds :type "Float (double-precision)") (InputAction :type "InputAction Object Reference" :default "/Game/Dev-Directory/Personal-Folders/Sebastian/InputActions/IA_FlyMove.IA_FlyMove"))
  (bind _returnvalue (`PawnMovementComponent.GetPawnOwner` (`self.characterMovementComponent`)))
  (bind (_returnvalue_roll _returnvalue_pitch _returnvalue_yaw) (`KismetMathLibrary.BreakRotator` (`Pawn.GetControlRotation` (`PawnMovementComponent.GetPawnOwner` (`self.characterMovementComponent`)))))
  (:`Triggered`
    (if (`self.isFlying`)
      (`Pawn.AddMovementInput` _returnvalue (`KismetMathLibrary.GetForwardVector` (`KismetMathLibrary.MakeRotator` 0.0 0.0 _returnvalue_yaw)) ActionValue_Y false)
      (`Pawn.AddControllerYawInput` _returnvalue ActionValue_X))))

(fn `FallAndGlide`
  (bind (_returnvalue_roll _returnvalue_pitch _returnvalue_yaw) (`KismetMathLibrary.BreakRotator` (`Controller.GetControlRotation` (`GameplayStatics.GetPlayerController` 0))))
  (`CharacterMovementComponent.AddForce` (`self.characterMovementComponent`) (- (* (`KismetMathLibrary.GetForwardVector` (`KismetMathLibrary.MakeRotator` 0.0 0.0 _returnvalue_yaw)) (`self.flightForwardGlideSpeed`)) (`KismetMathLibrary.MakeVector` 0.0 0.0 (`self.flightGravity`)))))

(fn `GetParentCharacterController`
  ;[1 1 1] Get and set Character Movement Component from Character Component
  (set `self.characterMovementComponent` (`Character.CharacterMovement` (`GameplayStatics.GetPlayerCharacter` 0))))

(fn `GroundCheck`
  (returns (groundCheck :type Boolean))
  (bind _returnvalue (`GameplayStatics.GetPlayerCharacter` 0))
  ;[1 1 1] Create box and check for collisions with terrain
  (bind (_outactors _returnvalue_2) (`KismetSystemLibrary.BoxOverlapActors` (- (`Actor.K2_GetActorLocation` _returnvalue) (0.0 0.0 100.0)) (25.0 25.0 15.0) (`|MakeArray` "ObjectTypeQuery1" :!type "EObjectTypeQuery Enum") null (`|MakeArray` _returnvalue :!type "Actor Object Reference")))
  ;[1 1 1] Return results of overlap check
  (return _returnvalue_2))