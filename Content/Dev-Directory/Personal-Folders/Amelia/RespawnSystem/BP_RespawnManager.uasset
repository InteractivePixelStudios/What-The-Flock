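; Respawn manager actor that tracks accessible nests as respawn points and handles which one is selected.
; It builds the list from BP_BaseNest actors on BeginPlay or refresh, and can default the selection to the one closest to the player.
; Cycling left or right and direct selection update the index and fire SelectedUpdate.
; Camera move events shift this actor horizontally, by teleport or timeline lerp, preserving its height.
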(event `self.ReceiveBeginPlay`
  ;[1 1 1] Gets all respawn points and puts them all in an array when they are accessible
  (bind _outactors (`GameplayStatics.GetAllActorsOfClass` "/Game/Dev-Directory/Personal-Folders/Sebastian/Blueprints/NestMechanics/BP_BaseNest.BP_BaseNest_C" :!label _label))
  (for _array_element _outactors
    (bind (_respawn_point_info_respawnpointname _respawn_point_info_isplayermade _respawn_point_info_isaccessible) (break `/Game/Dev-Directory/Personal-Folders/Amelia/RespawnSystem/RespawnSystem/S_RespawnPoint` (`/Game/Dev-Directory/Personal-Folders/Sebastian/Blueprints/NestMechanics/BP_BaseNest.Respawn Point Info` _array_element)))
    (if _respawn_point_info_isaccessible
      (`KismetArrayLibrary.Array_Add` (`self.Respawn Point Array`) _array_element))))

(event `Refresh Respawn Point Array`
  (`KismetArrayLibrary.Array_Clear` (`self.Respawn Point Array`))
  (goto _label))

(event `MoveCameraLerp`
  (params (NewLocation :type "Vector Structure"))
  (bind _returnvalue (`self.K2_GetActorLocation`))
  ;[1 1 1] 0-1 in 1 Second
  (bind (_direction _transition) (`Timeline|Timeline` :!via `PlayFromStart`)
    (:`Update`
      (`self.K2_SetActorLocation` (`KismetMathLibrary.MakeVector` (.x (`KismetMathLibrary.VLerp` _returnvalue NewLocation _transition)) (.y (`KismetMathLibrary.VLerp` _returnvalue NewLocation _transition)) (.z _returnvalue)) false true))))

(event `MoveCamera`
  (params (`New Location` :type "Vector Structure"))
  (`self.K2_SetActorLocation` (`KismetMathLibrary.MakeVector` (.x `New Location`) (.y `New Location`) (.z (`self.K2_GetActorLocation`))) false true))

(fn `CycleRespawnPointLeft`
  (returns (CurrentRespawnPoint :type "/Game/Dev-Directory/Personal-Folders/Sebastian/Blueprints/NestMechanics/BP_BaseNest Object Reference"))
  (bind _respawn_point_array (`self.Respawn Point Array`))
  ;[0.2611 1 0.2493] If index will drop below zero...
  (if (<= (`self.Selected Respawn Point Index`) 0)
    ;[0.2625 0.5528 1] ...Loop back to the top of the list
    (bind _output_get (set `self.Selected Respawn Point Index` (- (`KismetArrayLibrary.Array_Length` (`self.Respawn Point Array`)) 1)))
    (`self.SelectedUpdate` _output_get)
    ;[0.2625 0.5528 1] Getting the respawn point from the array
    (return (`|GetArrayItem` _respawn_point_array _output_get))
    (else
      ;[0.2625 0.5528 1] ...otherwise decrease Selected Index by 1
      (bind _output_get_2 (set `self.Selected Respawn Point Index` (- (`self.Selected Respawn Point Index`) 1)))
      (`self.SelectedUpdate` _output_get_2)
      (return (`|GetArrayItem` _respawn_point_array _output_get_2)))))

(fn `CycleRespawnPointRight`
  (returns (CurrentRespawnPoint :type "/Game/Dev-Directory/Personal-Folders/Sebastian/Blueprints/NestMechanics/BP_BaseNest Object Reference"))
  (bind _respawn_point_array (`self.Respawn Point Array`))
  (if (>= (`self.Selected Respawn Point Index`) (`KismetArrayLibrary.Array_Length` (`self.Respawn Point Array`)))
    ;[0.2625 0.5528 1] ...Loop back to the bottom of the list
    (bind _output_get (set `self.Selected Respawn Point Index` 0))
    (`self.SelectedUpdate` _output_get)
    (return (`|GetArrayItem` _respawn_point_array _output_get))
    (else
      ;[0.2625 0.5528 1] ...otherwise increase Selected Index by 1
      (bind _output_get_2 (set `self.Selected Respawn Point Index` (+ (`self.Selected Respawn Point Index`) 1)))
      (`self.SelectedUpdate` _output_get_2)
      (return (`|GetArrayItem` _respawn_point_array _output_get_2)))))

(fn `GetClosestRespawnPoint`
  (bind _returnvalue (`self.K2_GetActorLocation` (`GameplayStatics.GetPlayerPawn` 0)))
  (for (_array_element _array_index) (`self.Respawn Point Array`)
    ;[1 1 1] If first pass, reset default to 0
    (if (== _array_index 0)
      (set `self.Closest Respawn Point ` 0)
      (`KismetSystemLibrary.PrintText` "First point, defaulted to 0")
      (elif (> (`KismetMathLibrary.Vector_Distance` (`self.K2_GetActorLocation` (`|GetArrayItem` (`self.Respawn Point Array`) (`self.Closest Respawn Point `))) _returnvalue) (`KismetMathLibrary.Vector_Distance` _returnvalue (`self.K2_GetActorLocation` _array_element)))
        (bind _output_get (set `self.Closest Respawn Point ` _array_index))
        (`KismetSystemLibrary.PrintText` (`KismetTextLibrary.Conv_IntToText` _output_get))
        (else
          (`KismetSystemLibrary.PrintText` "Is not smaller")))))
  (set `self.Selected Respawn Point Index` (`self.Closest Respawn Point `)))

(fn `GetCurrentRespawnPoint`
  (returns (NewParam :type "/Game/Dev-Directory/Personal-Folders/Sebastian/Blueprints/NestMechanics/BP_BaseNest Object Reference"))
  (return (`|GetArrayItem` (`self.Respawn Point Array`) (`self.Selected Respawn Point Index`))))

(fn `SelectRespawnPoint`
  (params (`Selected Point` :type Integer))
  (bind _output_get (set `self.Selected Respawn Point Index` `Selected Point`))
  (`self.SelectedUpdate` _output_get))

(fn `UserConstructionScript`)