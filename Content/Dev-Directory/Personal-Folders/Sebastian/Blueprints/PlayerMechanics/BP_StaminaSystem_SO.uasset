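; Player stamina system that spends stamina through UseStamina, which reports success, and regenerates it up to a maximum.
; Recharging begins once SetStaminaToCharge is called, and Tick uses Delays to pace clamped RechargeStamina increments.
; Partial use waits before the first increment, while full depletion skips that wait and uses its own regen rate.
; Level-ups increment max stamina and print debug text.
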(event `self.ReceiveBeginPlay`
  ;[1 1 1] At start set stamina to max amount
  (set `self.stamina` (`self.maxStamina`)))

(event `self.ReceiveTick`
  (params (DeltaSeconds :type "Float (single-precision)"))
  (bind _regenticktime (`self.regenTickTime`))
  ;[1 1 1] Check if stamina can charge
  (if (`self.staminaCanCharge`)
    ;[1 1 1] If stamina is depleted charge faster
    (if (`self.staminaDepleted`)
      ;[1 1 1] Start regenerating after tick time amount with increased rate
      (`KismetSystemLibrary.Delay` _regenticktime)
      (`self.RechargeStamina` (`self.depletedStaminaRegenSpeed`))
      (else
        (if (`self.delayed`)
          ;[1 1 1] Once delayed regenerate at tick time
          (`KismetSystemLibrary.Delay` _regenticktime)
          (else
            ;[1 1 1] With stamina not depleted delay the first regeneration
            (`KismetSystemLibrary.Delay` (`self.timeToStartRegen`))
            (set `self.delayed` true)))
        ;[1 1 1] Recharge stamina at normal speed
        (`self.RechargeStamina` (`self.staminaRegenSpeed`))))))

(event `/Game/Dev-Directory/Personal-Folders/Jacob-EXP/XP-Content/BPI_XPInterface_JS.OnLevelUp`
  ;[1 1 1] On Level Up
  (bind _result (`/Engine/EditorBlueprintResources/StandardMacros.IncrementFloat` (`self.maxStamina`)) ; Increment Max by 1
    (:`  `
      (set `self.maxStamina` _result)
      (`KismetSystemLibrary.PrintString` "Max Stamina is now ")
      (`KismetSystemLibrary.PrintString` (`KismetStringLibrary.Conv_DoubleToString` (`self.maxStamina`)))
      (`KismetSystemLibrary.PrintString` "XP Stamina System"))))

(fn `RechargeStamina`
  (params (rechargeRate :type "Float (double-precision)"))
  ;[1 1 1] Add recharge rate to stamina and clamp to Max Stamina amount
  (set `self.stamina` (`KismetMathLibrary.FClamp` (+ (`self.stamina`) rechargeRate) 0.0 (`self.maxStamina`)))
  ;[1 1 1] Once max stamina reached, reset all bools for next use
  (if (== (`self.stamina`) (`self.maxStamina`))
    (set `self.staminaCanCharge` false)
    (set `self.staminaDepleted` false)
    (set `self.delayed` false)))

(fn `SetStaminaToCharge`
  ;[1 1 1] Function allows stamina to begin charging
  (set `self.staminaCanCharge` true))

(fn `UseStamina`
  (params (staminaUsed :type "Float (double-precision)"))
  (returns (usedStamina :type Boolean))
  (if (>= (- (`self.stamina`) staminaUsed) 0.0)
    ;[1 1 1] Reset all bools since stamina is being used
    (set `self.staminaCanCharge` false)
    (set `self.delayed` false)
    (set `self.staminaDepleted` false)
    ;[1 1 1] Subtract stamina used from stamina
    (bind _output_get (set `self.stamina` (- (`self.stamina`) staminaUsed)))
    ;[1 1 1] Check if stamina was fully depleted
    (if (== _output_get 0.0)
      (set `self.staminaDepleted` true))
    ;[1 1 1] Return true, stamina was used
    (return true)
    (else
      ;[1 1 1] Returns false, no stamina used
      (return false))))