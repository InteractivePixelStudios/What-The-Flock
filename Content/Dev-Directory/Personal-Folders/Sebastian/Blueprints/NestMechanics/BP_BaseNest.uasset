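; BP_BaseNest is a base actor for buildable nests that become player-named respawn points.
; While inactive, it asks its stick spawner to spawn the needed sticks for timed collection.
; NestBuilt activates the nest and opens a naming widget; SetNestName stores the respawn info and refreshes BP_RespawnManager's list.
; Material and visibility functions are empty here, and inventory access only prints a debug message.
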(fn `AccessInventory`
  (`KismetSystemLibrary.PrintString` "Spawning Inventory Widget"))

(fn `Input New Nest Name`
  (bind _returnvalue (`GameplayStatics.GetPlayerController` 0))
  (bind _namerref (`self.NamerRef`))
  (`/Engine/EditorBlueprintResources/StandardMacros.IsValid` (`self.NamerRef`)
    (:`Is Valid`
      _)
    (:`Is Not Valid`
      (bind _returnvalue_2 (`|CreateWidget` "/Game/Dev-Directory/Personal-Folders/Wesley/BluePrints_WK/UW_NestNamer_WK.UW_NestNamer_WK_C"))
      (set `self.NamerRef` _returnvalue_2)))
  (`UserWidget.AddToViewport` _namerref 0)
  (`WidgetBlueprintLibrary.SetInputMode_UIOnlyEx` _returnvalue _namerref)
  (set `/Game/Dev-Directory/Personal-Folders/Wesley/BluePrints_WK/UW_NestNamer_WK.NestToName` self _namerref)
  (set `PlayerController.bShowMouseCursor` true _returnvalue))

(fn `MakeInvisible`)

(fn `MakeVisible`)

(fn `NestBuilt`
  ;[1 1 1] Swaps from shimmer material and sets nest to active
  (`self.SwapMaterials`)
  (`self.SetActive` true)
  (`self.MakeVisible`)
  (`self.Input New Nest Name`))

(fn `SetActive`
  (params (`Is Active` :type Boolean))
  (set `self.Active` `Is Active`))

(fn `SetNestName`
  (params (NameInputText :type String))
  (set `self.Respawn Point Info` (make `/Game/Dev-Directory/Personal-Folders/Amelia/RespawnSystem/RespawnSystem/S_RespawnPoint` NameInputText true true))
  (bind _returnvalue (`GameplayStatics.GetActorOfClass` "/Game/Dev-Directory/Personal-Folders/Amelia/RespawnSystem/BP_RespawnManager.BP_RespawnManager_C"))
  (`/Game/Dev-Directory/Personal-Folders/Amelia/RespawnSystem/BP_RespawnManager.Refresh Respawn Point Array` _returnvalue))

(fn `SpawnSticks`
  (if (not (`self.Active`))
    (`KismetSystemLibrary.PrintString` "Spawning Sticks")
    (`/Game/Dev-Directory/Personal-Folders/Sebastian/Blueprints/NestMechanics/BP_StickSpawner.SpawnSticks` (`self.StickSpawnerLocation`) self 20.0 (`self.SticksNeeded`))))

(fn `SwapMaterials`)

(fn `UserConstructionScript`)