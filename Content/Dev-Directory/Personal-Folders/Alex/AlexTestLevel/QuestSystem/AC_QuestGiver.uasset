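; Quest giver component that lets its owning NPC offer a data table quest and present rewards when the player returns.
; InteractWithNPC checks the player's quest log, then either auto-accepts a new quest or opens the offer widget.
; For known quests, it queries the quest actor and shows the rewards widget if completed but not turned in.
; These successful interaction paths return the owner's display name.
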(event `/Game/Dev-Directory/Personal-Folders/Alex/AlexTestLevel/QuestSystem/BPI_QuestInteractionInterface.LookAtNPC`)

(fn `DisplayQuest`
  (bind (_questdata_datatable _questdata_rowname) (break `DataTableRowHandle` (`self.QuestData`)))
  ;[0.6875 0.1683 0.1683 0.7216] Prints quest name from data table row and shows the quest giver widget
  (bind _returnvalue (`|GetDataTableRow` _questdata_datatable _questdata_rowname)
    (:`then`
      (bind _returnvalue_2 (`|CreateWidget` "/Game/Dev-Directory/Personal-Folders/Alex/AlexTestLevel/QuestSystem/UI/WBP_QuestGiverWidget.WBP_QuestGiverWidget_C" null _returnvalue _questdata_rowname))
      (`UserWidget.AddToViewport` _returnvalue_2 0))))

(fn `DisplayRewards`
  (bind (_questdata_datatable _questdata_rowname) (break `DataTableRowHandle` (`self.QuestData`)))
  ;[0.6875 0.1683 0.1683 0.7216] Displays the quest rewards widget
  (bind _returnvalue (`|GetDataTableRow` _questdata_datatable _questdata_rowname)
    (:`then`
      (bind _returnvalue_2 (`|CreateWidget` "/Game/Dev-Directory/Personal-Folders/Alex/AlexTestLevel/QuestSystem/UI/WBP_QuestRewardsWidget.WBP_QuestRewardsWidget_C" null _returnvalue _questdata_rowname))
      (`UserWidget.AddToViewport` _returnvalue_2 0))))

(fn `InteractWithNPC`
  (returns (ObjectiveID :type String))
  (bind (_questdata_datatable _questdata_rowname) (break `DataTableRowHandle` (`self.QuestData`)))
  (bind (_questdata_datatable_2 _questdata_rowname_2) (break `DataTableRowHandle` (`self.QuestData`)))
  (bind (_questdata_datatable_3 _questdata_rowname_3) (break `DataTableRowHandle` (`self.QuestData`)))
  (bind (_questdata_datatable_4 _questdata_rowname_4) (break `DataTableRowHandle` (`self.QuestData`)))
  (bind _returnvalue (`KismetSystemLibrary.GetDisplayName` (`self.GetOwner`)))
  (bind _returnvalue_2 (`Actor.GetComponentByClass` (`GameplayStatics.GetPlayerCharacter` 0) "/Game/Dev-Directory/Personal-Folders/Alex/AlexTestLevel/QuestSystem/AC_QuestLog.AC_QuestLog_C"))
  (bind _ac_questlog (`/Game/Dev-Directory/Personal-Folders/Alex/AlexTestLevel/PlayerCharacter/BP_PigeonCharacter_AB.AC_QuestLog` (`/Game/Dev-Directory/Personal-Folders/Alex/AlexTestLevel/QuestSystem/FL_QuestFunctionLibrary.GetPigeonCharacter`)))
  ;[0.2314 0.1137 0.5529] Checks is they are both NOT TRUE
  (if (and (not (`/Game/Dev-Directory/Personal-Folders/Alex/AlexTestLevel/QuestSystem/AC_QuestLog.QueryActiveQuest` _ac_questlog _questdata_rowname_2)) (not (`/Game/Dev-Directory/Personal-Folders/Alex/AlexTestLevel/QuestSystem/AC_QuestLog.QueryCompletedQuest` _ac_questlog _questdata_rowname_2)))
    ;[0.2314 0.1137 0.5529] Checks to see if the quest is set to AutoAccept
    (bind _returnvalue_3 (`|GetDataTableRow` "/Game/Dev-Directory/Personal-Folders/Alex/AlexTestLevel/QuestSystem/DT_QuestData.DT_QuestData" _questdata_rowname_3)
      (:`then`
        (if (`.AutoAccept_16_620952754D7D2828804DCCBFFE1AD1EB` (break `/Game/Dev-Directory/Personal-Folders/Alex/AlexTestLevel/QuestSystem/S_QuestDetails` _returnvalue_3))
          ;[0.6875 0.1683 0.1683 0.7216] Gets the quest log component from the player and adds a new quest
          (`/Engine/EditorBlueprintResources/StandardMacros.IsValid` _returnvalue_2
            (:`Is Valid`
              (`/Game/Dev-Directory/Personal-Folders/Alex/AlexTestLevel/QuestSystem/AC_QuestLog.AddNewQuest` _returnvalue_2 _questdata_rowname_4)
              (return (`KismetSystemLibrary.GetDisplayName` (`self.GetOwner`)))))
          (else
            ;[0.6875 0.1683 0.1683 0.7216] Displays quest if true
            (`self.DisplayQuest`)
            (return _returnvalue)))))
    (else
      ;[0.2314 0.1137 0.5529] Displays the rewards when the quest is completed and the player interacts with the quest giver
      (bind _array_element (`/Game/Dev-Directory/Personal-Folders/Alex/AlexTestLevel/QuestSystem/AC_QuestLog.GetQuestActor` (`/Game/Dev-Directory/Personal-Folders/Alex/AlexTestLevel/PlayerCharacter/BP_PigeonCharacter_AB.AC_QuestLog` (`/Game/Dev-Directory/Personal-Folders/Alex/AlexTestLevel/QuestSystem/FL_QuestFunctionLibrary.GetPigeonCharacter`)) _questdata_rowname))
      (if (and (`/Game/Dev-Directory/Personal-Folders/Alex/AlexTestLevel/QuestSystem/BP_QuestsBase.isCompleted` _array_element) (not (`/Game/Dev-Directory/Personal-Folders/Alex/AlexTestLevel/QuestSystem/BP_QuestsBase.isQuestTurnedIn` _array_element)))
        (`self.DisplayRewards`)
        (return _returnvalue)))))