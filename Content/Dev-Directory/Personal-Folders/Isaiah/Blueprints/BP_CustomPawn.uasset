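; Player pawn that owns the on-screen HUD and a toggleable world map.
; On BeginPlay it creates both widgets, hides the map and its arrow component, and copies Health, Stamina, Dooky and EXP from BPPlayerStats into listener variables once.
; Pressing M flips between map and HUD, showing the WorldMapArrow only while the map is open.
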(event `Key|M`
  (params (Key :type "Key Structure"))
  ;[1 1 1] Button Listeners
  (:`Pressed`
    (if (`self.Is Map Open`)
      (`self.Toggle World Map OFF`)
      (else
        (`self.Toggle World Map ON`)))))

(event `self.ReceiveBeginPlay`
  (`self.CreateHUD`)
  (`self.UpdateHUD`)
  (`SceneComponent.SetHiddenInGame` (`self.WorldMap_Arrow`) true false))

(event `UpdateHUD`
  (set `self.HealthListener` (`/Game/Dev-Directory/Personal-Folders/Isaiah/Blueprints/BP_PlayerStats.Health` (`self.BP_PlayerStats`)))
  (set `self.StaminaListener` (`/Game/Dev-Directory/Personal-Folders/Isaiah/Blueprints/BP_PlayerStats.Stamina` (`self.BP_PlayerStats`)))
  (set `self.DookyListener` (`/Game/Dev-Directory/Personal-Folders/Isaiah/Blueprints/BP_PlayerStats.Dooky` (`self.BP_PlayerStats`)))
  (set `self.EXPListener` (`/Game/Dev-Directory/Personal-Folders/Isaiah/Blueprints/BP_PlayerStats.EXP` (`self.BP_PlayerStats`))))

(event `CreateHUD`
  (bind _returnvalue (`|CreateWidget` "/Game/Dev-Directory/Personal-Folders/Isaiah/PlayerHUD_Widget.PlayerHUD_Widget_C" (`GameplayStatics.GetPlayerController` 0)))
  (bind _output_get (set `self.Player HUD` _returnvalue))
  (`UserWidget.AddToViewport` _output_get 0)
  (bind _returnvalue_2 (`|CreateWidget` "/Game/Dev-Directory/Personal-Folders/Isaiah/WorldMap_Widget.WorldMap_Widget_C" (`GameplayStatics.GetPlayerController` 0)))
  (bind _output_get_2 (set `self.WorldMap` _returnvalue_2))
  (`UserWidget.AddToViewport` _output_get_2 0)
  (`Widget.SetVisibility` (`self.WorldMap`) "Hidden")
  (set `self.Is Map Open` false)
  (`KismetSystemLibrary.PrintText` "HUD and World Map have been created."))

(event `Toggle World Map ON`
  (set `self.Is Map Open` true)
  (`Widget.SetVisibility` (`self.Player HUD`) "Hidden")
  (`SceneComponent.SetHiddenInGame` (`self.WorldMap_Arrow`) false false)
  (`Widget.SetVisibility` (`self.WorldMap`) "Visible")
  (`KismetSystemLibrary.PrintText` "Toggled Map On"))

(event `Toggle World Map OFF`
  (set `self.Is Map Open` false)
  (`Widget.SetVisibility` (`self.WorldMap`) "Hidden")
  (`SceneComponent.SetHiddenInGame` (`self.WorldMap_Arrow`) true false)
  (`Widget.SetVisibility` (`self.Player HUD`) "Visible")
  (`KismetSystemLibrary.PrintText` "Toggle Map Off"))

(fn `UserConstructionScript`)